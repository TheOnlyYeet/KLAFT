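; Camera actor that positions itself at an offset from a given player pawn and can animate back to that spot.
; GetResetLocation adds the X and Z of RelativPositionToPlayer along the camera's own forward and up vectors to the pawn's location.
; FixCameraLocation snaps there, while SetupPointForReset caches start and end points and lerps between them on a timeline.
; MoveCameraForReset applies the same lerp with an externally supplied alpha.
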(event Custom|SetupPointForReset
  (params (RefPawn :type Pawn%20Object%20Reference))
  (Variables|Default|SetEndPoint (CallFunction|GetResetLocation RefPawn))
  (Variables|Default|SetStartPoint (Transformation|GetActorLocation))
  (bind _newtrack_0 (Timeline|ANimResetCamera PlayFromStart)
    (:Update
      (Transformation|SetActorLocation (Math|Vector|Lerp(Vector) (Variables|Default|GetStartPoint) (Variables|Default|GetEndPoint) _newtrack_0) false false))))

(event Custom|FixCameraLocation
  (params (RefPlayer :type Pawn%20Object%20Reference))
  (Transformation|SetActorLocation (CallFunction|GetResetLocation RefPlayer) false false))

(event Custom|MoveCameraForReset
  (params (Alpha :type Float%20%28single-precision%29))
  (Transformation|SetActorLocation (Math|Vector|Lerp(Vector) (Variables|Default|GetStartPoint) (Variables|Default|GetEndPoint) Alpha) false false))

(fn ConstructionScript)

(fn GetResetLocation
  (params (RefPawn :type Pawn%20Object%20Reference))
  (bind _relativpositiontoplayer (Variables|Default|GetRelativPositionToPlayer))
  (return (+ (Transformation|GetActorLocation RefPawn) (+ (* (Transformation|GetActorForwardVector) (.x _relativpositiontoplayer)) (* (Transformation|GetActorUpVector) (.z _relativpositiontoplayer))))))