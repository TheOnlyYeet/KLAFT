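; Replicated board tile for a grid map, holding terrain type, enemy slots, shop card and gem lists, and movement state.
; Construction builds two back-to-back child tiles on a pivot, sets movement rules by type and picks monster-road enemies by region.
; A server-triggered timeline flips the pivot while toggling face visibility, advances the tile index, then spawns or reuses that slot's enemy to start a fight.
; OnRep functions drive monster and player icons, and events spawn per-type lighting.
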(event Custom|S_SpawnEnemy
  (params (PC :type PC%20Klaft%20Game%20Object%20Reference))
  (Utilities|IsValid (Variables|Default|GetRefEnemyPawn)
    (:Is%20Valid
      (Default|SFightSystemModuleInitialization PC (Variables|Default|GetRefEnemyPawn)))
    (:Is%20Not%20Valid
      (bind _returnvalue (Game|SpawnActorfromClass (.ClassEnemy_T1 (CallFunction|GetInfoTileIndex (Variables|Default|GetIndexTileType?))) (Math|Conversions|ToTransform(Vector) (+ (Transformation|GetActorLocation) "0, 0,96.000000")) "Undefined" 0 0))
      (bind _output_get (Variables|Default|SetRefEnemyPawn _returnvalue))
      (Default|SRotateEnemy _output_get (Transformation|GetActorLocation (Pawn|GetControlledPawn PC)))
      (Default|SFightSystemModuleInitialization PC (Variables|Default|GetRefEnemyPawn)))))

(event Custom|S_InitializeAnimTile
  (params (PC :type PC%20Klaft%20Game%20Object%20Reference))
  (bind _pivottile (Variables|Default|GetPivotTile))
  (if (not (Variables|Default|GetAnimationIsPlaying?))
    (Variables|Default|SetAnimationIsPlaying? true)
    (Variables|Default|SetRelative%20Rotation (Transformation|GetWorldRotation _pivottile))
    (bind _isa (Utilities|FlowControl|FlipFlop)
      (:A
        _)
      (:B
        _))
    (CallFunction|OptimizationViewPortTile _isa)
    (bind _percentanimation (Timeline|Animation PlayFromStart)
      (:Update
        (Transformation|SetWorldRotation _pivottile (Math|Rotator|Lerp(Rotator) (Variables|Default|GetRelative%20Rotation) (Math|Rotator|CombineRotators (Variables|Default|GetRelative%20Rotation) "180.000000, 0, 0") _percentanimation true) false false))
      (:Finished
        (Variables|Default|SetIndexTileType? (Math|Integer|Clamp(Integer) (+ (Variables|Default|GetIndexTileType?) 1) 1 5))
        (Variables|Default|SetRelative%20Rotation (Transformation|GetActorRotation))
        (Variables|Default|SetAnimationIsPlaying? false)
        (if (Variables|SettingsBaseTile|GetTournoiMode?)
          (Default|SSetTournoiMode PC true))
        (if (.Enemy_T1 (CallFunction|GetInfoTileIndex (Variables|Default|GetIndexTileType?)))
          (CallFunction|SSpawnEnemy PC)
          (Transformation|SetWorldRotation (Variables|Default|GetIconPOssibleMove) "180.000000, 0, 0" true false))))))

(event Custom|S_SpawnLight
  (params (TypeTyle :type EListTypeTile%20Enum :default "NewEnumerator0"))
  (CallFunction|MSpawnLight TypeTyle))

(event Custom|S_RemoveLight
  (Actor|DestroyActor (Variables|Default|GetRefLighting)))

(event Custom|M_SpawnLight
  (params (Index :type EListTypeTile%20Enum :default "NewEnumerator0"))
  (bind _returnvalue (Game|SpawnActorfromClass (Utilities|Select :Index Index :NewEnumerator0 "/Game/Kyllian/Valid/Assets/Lights/BP_Lights_CaseForet.BP_Lights_CaseForet_C" :NewEnumerator1 "/Game/Kyllian/Valid/Assets/Lights/BP_Lights_CaseMonstre.BP_Lights_CaseMonstre_C" :NewEnumerator2 "/Game/Kyllian/Valid/Assets/Lights/BP_Lights_CasePlaine.BP_Lights_CasePlaine_C" :NewEnumerator3 "/Game/Kyllian/Valid/Assets/Lights/BP_Lights_CaseMontagne.BP_Lights_CaseMontagne_C" :NewEnumerator4 "/Game/Kyllian/Valid/Assets/Lights/BP_Lights_CaseCristallerie.BP_Lights_CaseCristallerie_C" :NewEnumerator5 "/Game/Kyllian/Valid/Assets/Lights/BP_Lights_CaseRoulotte.BP_Lights_CaseRoulotte_C" :NewEnumerator6 "/Game/Kyllian/Valid/Assets/Lights/BP_Lights_CasePlaine.BP_Lights_CasePlaine_C" :NewEnumerator7 "/Game/Kyllian/Valid/Assets/Lights/BP_Lights_CaseSyncristal_Gauche.BP_Lights_CaseSyncristal_Gauche_C" :NewEnumerator8 "/Game/Kyllian/Valid/Assets/Lights/BP_Lights_CaseSyncristal.BP_Lights_CaseSyncristal_C" :NewEnumerator9 "/Game/Kyllian/Valid/Assets/Lights/BP_Lights_CaseForet.BP_Lights_CaseForet_C" :NewEnumerator10 "/Game/Kyllian/Valid/Assets/Lights/BP_Lights_CaseForet.BP_Lights_CaseForet_C") (Math|Transform|MakeTransform (Transformation|GetActorLocation self) "0, 0, 0" "1,1,1") "Undefined" 0 0))
  (Variables|Default|SetRefLighting _returnvalue))

(event Custom|M_SetGemmeList
  (params (ListGemmeInShop :type Array%20of%20ST%20Carac%20Player%202%20Structures))
  (Variables|SettingsshopGemme|SetListGemmeInShop ListGemmeInShop))

(event Custom|M_Construction
  (if (Variables|SettingsBaseTile|GetTransitionTile?)
    (Variables|Default|SetIndexTransition (+ (Variables|SettingsBaseTile|GetRegionIndex) 1)))
  (Utilities|ConstructionStr))

(event Custom|S_ConstructionScript
  (CallFunction|MConstruction))

(event Custom|S_SetGemmeList
  (params (ListGemmeInShop :type Array%20of%20ST%20Carac%20Player%202%20Structures))
  (CallFunction|MSetGemmeList ListGemmeInShop))

(event Custom|M_SetCardList
  (params (LIstCardInShop :type Array%20of%20ST%20Cards%20Infos%20Structures))
  (Variables|SettingsRoulotte|SetLIstCardInShop LIstCardInShop))

(event Custom|S_SetCardList
  (params (LIstCardInShop :type Array%20of%20ST%20Cards%20Infos%20Structures))
  (CallFunction|MSetCardList LIstCardInShop))

(event EventBeginPlay
  (Components|Timeline|SetPlayRate (Variables|Default|GetAnimation) (/ 1.0 (Variables|SettingsBaseTile|GetDurationAnimation)))
  (Networking|SwitchHasAuthority
    (:Authority
      (CallFunction|SConstructionScript)
      (if (Utilities|Enum|Equal(Enum) (.TypeTile (CallFunction|GetInfoTileIndex)) "NewEnumerator4")
        (Variables|SettingsBaseTile|SetRespawnPossible true)))))

(fn ConstructionScript
  (if (Variables|SettingsBaseTile|GetTransitionTile?)
    (Variables|Default|SetIndexTransition (+ (Variables|SettingsBaseTile|GetRegionIndex) 1)))
  (Utilities|ConstructionStr))

(fn SetupConstruction
  (Default|SetupTile (.AsBP%20Tileversoin%202 (Utilities|Casting|CastToBP_Tileversoin2 (Variables|/Script/Engine.ChildActorComponent|GetChildActor (Variables|Default|GetTile2)))) (Variables|SettingsT2|GetTypeTile_2))
  (Default|SetupTile (.AsBP%20Tileversoin%202 (Utilities|Casting|CastToBP_Tileversoin2 (Variables|/Script/Engine.ChildActorComponent|GetChildActor (Variables|Default|GetTile1)))) (Variables|SettingsT1|GetTypeTile)))

(fn OnRepRefEnemyPawn
  (Utilities|IsValid (Variables|Default|GetRefEnemyPawn)
    (:Is%20Valid
      (Variables|Default|SetEnemyIsHere? true))
    (:Is%20Not%20Valid
      (Variables|Default|SetEnemyIsHere? false))))

(fn OnRepPlayerIsHere?
  (bind _iconpossiblemove (Variables|Default|GetIconPOssibleMove))
  (if (Variables|Default|GetPlayerIsHere?)
    (Rendering|SetVisibility _iconpossiblemove true true)
    (else
      (Rendering|SetVisibility _iconpossiblemove false true))))

(fn OnRepPOssibletoMove?)

(fn OnRepTransitionTile?)

(fn OnRepIndexTileType?)

(fn GetInfoTileIndex
  (params (Selection :type Integer))
  (switch int Selection
    (:0
      (return "NewEnumerator0" false 0))
    (:1
      (return (Variables|SettingsT1|GetTypeTile) (Variables|SettingsT1|GetEnemy_T1) (Variables|SettingsT1|GetClassEnemy_T1)))
    (:2
      (return (Variables|SettingsT2|GetTypeTile_2) (Variables|SettingsT2|GetEnemy_T2) (Variables|SettingsT2|GetClassEnemy_T2)))
    (:3
      (return (Variables|SettingsT3|GetTypeTile_3) (Variables|SettingsT3|GetEnemy_T3) (Variables|SettingsT3|GetClassEnemy_T3)))
    (:4
      (return (Variables|SettingsT4|GetTypeTile_4) (Variables|SettingsT4|GetEnemy_T4) (Variables|SettingsT4|GetClassEnemy_T4)))
    (:5
      (return (Variables|SettingsT5|GetTypeTile_5) (Variables|SettingsT5|GetEnemy_T5) (Variables|SettingsT5|GetClassEnemy_T5)))))

(fn OnRepListGemmeinShop)

(fn OnRepLIstCardinShop)

(fn OnRepRefLighting)

(fn OnRepNbItemCreate)

(fn OnRepEnemyIsHere?
  (bind _iconmonster (Variables|Default|GetIconMonster))
  (if (Variables|Default|GetEnemyIsHere?)
    (Rendering|SetVisibility _iconmonster true true)
    (else
      (Rendering|SetVisibility _iconmonster false true))))

(fn OnRepRespawnPossible)

(fn OnRepTournoiMode?)

(fn OnRepRefPlayerIsHere
  (if (not (Variables|Default|GetPlayerIsHere?))
    (Variables|Default|SetRefPlayerIsHere 0)))

(fn OptimizationViewPortTile
  (params (Is%20A :type Boolean))
  (Rendering|SetVisibility (select Is%20A (Variables|Default|GetTile2) (Variables|Default|GetTile1)) true true)
  (Rendering|SetVisibility (select Is%20A (Variables|Default|GetTile1) (Variables|Default|GetTile2)) false true))