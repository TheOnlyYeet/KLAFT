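; Grid cell actor that holds two back-to-back child tiles on a pivot and can flip over to swap the visible face.
; Construction spawns and types both tiles, links them back to the cell, and sets move and animation flags for special types.
; On BeginPlay the authority reruns construction through server-to-multicast events.
; The flip is also multicast, using a timeline to rotate the whole actor 180 degrees, guarded against overlapping plays.
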(event Custom|M_PlayAnimation
  (bind _returnvalue (Transformation|GetActorRotation))
  (if (not (Variables|Default|GetAnimationIsPlaying?))
    (Variables|Default|SetAnimationIsPlaying? true)
    (Variables|Default|SetRelative%20Rotation _returnvalue)
    (Utilities|FlowControl|FlipFlop
      (:A
        (bind _percentanimation (Timeline|Animation PlayFromStart)
          (:Update
            (Transformation|SetActorRotation (Math|Rotator|Lerp(Rotator) (Variables|Default|GetRelative%20Rotation) (Math|Rotator|CombineRotators (Variables|Default|GetRelative%20Rotation) "180.000000, 0, 0") _percentanimation true)))
          (:Finished
            (Variables|Default|SetRelative%20Rotation _returnvalue)
            (Variables|Default|SetAnimationIsPlaying? false))))
      (:B
        (Timeline|Animation PlayFromStart)))))

(event Custom|S_InitializeAnimTile
  (CallFunction|MPlayAnimation))

(event Custom|M_Construction
  (if (Variables|SettingsBaseTile|GetTransitionTile?)
    (Variables|Default|SetIndexTransition (+ (Variables|SettingsBaseTile|GetRegionIndex) 1)))
  (Utilities|ConstructionStr))

(event Custom|S_ConstructionScript
  (CallFunction|MConstruction))

(event EventBeginPlay
  (Components|Timeline|SetPlayRate (Variables|Default|GetAnimation) (/ 1.0 (Variables|SettingsBaseTile|GetDurationAnimation)))
  (Networking|SwitchHasAuthority
    (:Authority
      (CallFunction|SConstructionScript))))

(fn ConstructionScript
  (if (Variables|SettingsBaseTile|GetTransitionTile?)
    (Variables|Default|SetIndexTransition (+ (Variables|SettingsBaseTile|GetRegionIndex) 1)))
  (Utilities|ConstructionStr))

(fn SetupConstruction
  (Default|SetupTile (.AsBP%20Tileversoin%202 (Utilities|Casting|CastToBP_Tileversoin2 (Variables|/Script/Engine.ChildActorComponent|GetChildActor (Variables|Default|GetTile2)))) (Variables|SettingsT2|GetTypeTile_2))
  (Default|SetupTile (.AsBP%20Tileversoin%202 (Utilities|Casting|CastToBP_Tileversoin2 (Variables|/Script/Engine.ChildActorComponent|GetChildActor (Variables|Default|GetTile1)))) (Variables|SettingsT1|GetTypeTile)))