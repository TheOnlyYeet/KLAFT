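; Lobby player controller that shows a loading widget during its lifetime and handles spawning and possessing the player's character.
; S_SpawnCharacter reads the character selection and player index from BP_PMM_Instance and forwards them to a server spawn event.
; That event claims a PlayerStart by tagging it "Found", then spawns there and possesses the result.
; The spawn node shows no class, and the BP_Character index assignment is disconnected.
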(event Custom|S_SpawnCharacterServer
  (params (ClassCharacter :type BP%20Character%20Class%20Reference))
  (bind _outactors (Actor|GetAllActorsOfClass "/Script/Engine.PlayerStart"))
  (bind _array_element (Utilities|Array|ForEachLoopwithBreak _outactors :!label _label)
    (:LoopBody
      (if (Utilities|Name|NotEqual(Name) (Variables|/Script/Engine.PlayerStart|GetPlayerStartTag _array_element) "Found")
        (Variables|/Script/Engine.PlayerStart|SetPlayerStartTag _array_element "Found")
        (goto _label Break)))
    (:Completed
      (bind _returnvalue (Game|SpawnActorfromClass 0 (Math|Transform|MakeTransform (.location (Transformation|GetActorTransform _array_element)) (.rotation (Transformation|GetActorTransform _array_element)) "1,1,1") "AlwaysSpawn" 0 0))
      (Pawn|Possess _returnvalue))))

(event Custom|S_SpawnCharacter
  (bind _asbp_pmm_instance (Utilities|Casting|CastToBP_PMM_Instance (Game|GetGameInstance)))
  (CallFunction|SSpawnCharacterServer (Variables|/Game/CoreKlaft/BP_PMM_Instance.BP_PMM_Instance_C|GetCharacterSelection _asbp_pmm_instance) (Variables|/Game/CoreKlaft/BP_PMM_Instance.BP_PMM_Instance_C|GetIndexPlayer _asbp_pmm_instance)))

(event EventBeginPlay
  (bind _returnvalue (UserInterface|CreateWidget "/Game/ProMainMenu/Widgets/WD_LobbyLoadingPlayer.WD_LobbyLoadingPlayer_C"))
  (UserInterface|Viewport|AddtoViewport _returnvalue 0))

(event EventEndPlay
  (params (EndPlayReason :type EEndPlayReason%20Enum :default "Destroyed"))
  (Widget|RemovefromParent (stale EventBeginPlay _returnvalue)))

(fn ConstructionScript)