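; PC_KlaftGame is the networked player controller for Klaft's turn-based tile game, handling character spawning, camera panning and turn actions.
; The game state's active-player event sets IsMyTurn, gating clicks that send the tile under the cursor to S_ActionPlayer.
; That validates the tile, then spends PA to move or ends the turn at zero.
; Fight modules resolve posture, card and stat comparisons, but ConditionForAction's hardwired branch never reaches Enemy Here.
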(event Custom|S_RespawnCharacter
  (bind _asbp_pmm_instance (Utilities|Casting|CastToBP_PMM_Instance (Game|GetGameInstance)))
  (Default|RespawnCharacter (.AsGM%20Klaft%20Game (Utilities|Casting|CastToGM_KlaftGame (Game|GetGameMode))) (Variables|/Game/CoreKlaft/BP_PMM_Instance.BP_PMM_Instance_C|GetCharacterSelection _asbp_pmm_instance) self))

(event Custom|C_SpawnCharacter
  (params (Controller :type Controller%20Object%20Reference))
  ;[1 1 1] reseau
  (Variables|Default|SetIsMyTurn? false)
  (bind _asbp_pmm_instance (Utilities|Casting|CastToBP_PMM_Instance (Game|GetGameInstance)))
  (CallFunction|SSpawnCharacterServer (Variables|/Game/CoreKlaft/BP_PMM_Instance.BP_PMM_Instance_C|GetCharacterSelection _asbp_pmm_instance) Controller))

(event Custom|S_SpawnCharacterServer
  (params (ClassCharacter :type BP%20Character%20Class%20Reference) (Target :type Controller%20Object%20Reference))
  ;[1 1 1] reseau
  (bind _outactors (Actor|GetAllActorsOfClass "/Script/Engine.PlayerStart"))
  (bind _array_element (Utilities|Array|ForEachLoopwithBreak _outactors :!label _label)
    (:LoopBody
      (if (Utilities|Name|NotEqual(Name) (Variables|/Script/Engine.PlayerStart|GetPlayerStartTag _array_element) "Found")
        (Variables|/Script/Engine.PlayerStart|SetPlayerStartTag _array_element "Found")
        (goto _label Break)))
    (:Completed
      (bind _returnvalue (Game|SpawnActorfromClass ClassCharacter (Math|Transform|MakeTransform (.location (Transformation|GetActorTransform _array_element)) (.rotation (Transformation|GetActorTransform _array_element)) "1,1,1") "AlwaysSpawn" 0 0 0))
      (Pawn|Possess self _returnvalue))))

(event EventBeginPlay
  (Input|SetInputModeGameOnly self)
  (EventDispatchers|BindEventtoOnActivePlayerSetIndex (.AsGMS%20Klaft (Utilities|Casting|CastToGMS_Klaft (Game|GetGameState))) (EventDispatchers|CreateEvent :!event PCKlaftGameAutoGenFunc)))

(event Custom|C_CameraMoving
  (params (AxisValue :type Float%20%28single-precision%29) (Forward? :type Boolean) (IntensitySpeed :type Float%20%28single-precision%29))
  (bind _asbp_character (CallFunction|GetPlayerPawn))
  (bind _refcamera (Variables|/Game/CoreKlaft/BP_Character.BP_Character_C|GetRefCamera _asbp_character))
  (Transformation|SetActorLocation _refcamera (+ (Transformation|GetActorLocation _refcamera) (* (* (select Forward? (Transformation|GetActorForwardVector _refcamera) (Transformation|GetActorRightVector _refcamera)) IntensitySpeed) AxisValue)) false false))

(event Input|AxisEvents|InputAxisCameraAxisMoveForward
  (params (AxisValue :type Float%20%28single-precision%29))
  (CallFunction|CCameraMoving AxisValue true 1e+01))

(event Input|AxisEvents|InputAxisCameraAxisMoveRight
  (params (AxisValue :type Float%20%28single-precision%29))
  (CallFunction|CCameraMoving AxisValue false 1e+01))

(event Input|AxisEvents|InputAxisCameraAxisZoom
  (params (AxisValue :type Float%20%28single-precision%29)))

(event Input|MouseEvents|LeftMouseButton
  (params (Key :type Key%20Structure :default "None"))
  (:Pressed
    (if (Variables|Default|GetIsMyTurn?)
      (if (not (Variables|Default|GetActionLaunch))
        (Variables|Default|SetActionLaunch true)
        (bind _hittilecontenerref (CallFunction|GetHitTilefromCursor))
        (CallFunction|SActionPlayer _hittilecontenerref)))))

(event Input|KeyboardEvents|T
  (params (Key :type Key%20Structure :default "None"))
  (bind _asbp_character (CallFunction|GetPlayerPawn))
  (:Pressed
    (Default|FixCameraLocation (Variables|/Game/CoreKlaft/BP_Character.BP_Character_C|GetRefCamera _asbp_character) _asbp_character)))

(event Custom|C_SetPlayerIndex
  (params (Index :type Integer))
  (Variables|Default|SetIndexPlayer Index)
  ;[0 0.976 1] Create widget Possible
  (bind _returnvalue (UserInterface|CreateWidget "/Game/CoreKlaft/WD_TestTourdejeu.WD_TestTourdejeu_C" 0 self (Variables|Default|GetIndexPlayer)))
  (UserInterface|Viewport|AddtoViewport _returnvalue 0))

(event Custom|S_FightSystemModule
  (params (RefEnemy :type BP%20Character%20Enemy%20Object%20Reference) (TileContenerRef :type BP%20Tile%20Contener%20Grid%20Object%20Reference))
  (bind _asbp_character (CallFunction|GetPlayerPawn))
  ;[1 1 1] MODULES
  ;;[1 1 1] Player Vs Mob
  (Utilities|IsValid RefEnemy
    (:Is%20Valid
      (Utilities|ModuleFight (Variables|/Game/CoreKlaft/BP_Character.BP_Character_C|GetRefInfoPlayer _asbp_character) (Variables|/Game/CoreKlaft/BP_CharacterEnemy.BP_CharacterEnemy_C|GetRefInfoEnemy RefEnemy)
        (:Win
          (Actor|DestroyActor RefEnemy)
          (CallFunction|SMovingPlayer (Transformation|GetActorLocation TileContenerRef)))
        (:Lose
          (Actor|DestroyActor _asbp_character))))))

(event Custom|S_LaunchAnimationTile
  (params (RefTileContener :type BP%20Tile%20Contener%20Grid%20Object%20Reference))
  (Default|SInitializeAnimTile RefTileContener self))

(event Custom|S_MovingPlayer
  (params (NewLocationPoint :type Vector))
  (Default|SMovingInializationAction (CallFunction|GetPlayerPawn) NewLocationPoint))

(event Custom|S_ActionPlayer
  (params (TargetTileContener :type BP%20Tile%20Contener%20Grid%20Object%20Reference))
  (bind _tilecontenertarget (Utilities|ConditionforAction TargetTileContener)
    (:ValidMovement
      (Utilities|NewMacro0
        (:NoPaForMove
          (bind _asgms_klaft (Utilities|Casting|CastToGMS_Klaft (Game|GetGameState)))
          (Default|SEndPlayerTurn _asgms_klaft))
        (:MovePossible
          (CallFunction|SLaunchAnimationTile _tilecontenertarget)
          (CallFunction|SMovingPlayer (Transformation|GetActorLocation _tilecontenertarget)))))
    (:EnemyHere
      (CallFunction|SFightSystemModule (Variables|/Game/Klaft/Blueprint/BP_TileContenerGrid.BP_TileContenerGrid_C|GetRefEnemyPawn _tilecontenertarget) _tilecontenertarget))))

(event Custom|S_EndPlayerTurn
  (Default|SEndPlayerTurn (.AsGMS%20Klaft (Utilities|Casting|CastToGMS_Klaft (Game|GetGameState)))))

(event Custom|S_ListPlayer
  (CallFunction|FoundPlayerController))

(event Custom|S_PASystemModule)

(event Input|KeyboardEvents|P
  (params (Key :type Key%20Structure :default "None"))
  (:Pressed
    (CallFunction|SListPlayer)))

(event Custom|S_AddDelGemme
  (params (Add? :type Boolean) (Value :type Integer))
  ;[1 0 0.1556] Comment
  ;;[1 0 0.1556] Comment
  (Variables|Default|SetNbGemme (select Add? (+ (Variables|Default|GetNbGemme) Value) (- (Variables|Default|GetNbGemme) Value))))

(event Custom|S_AddRemoveCardList
  (params (AddCardInList? :type Boolean) (Item :type ST%20Cards%20Infos%20Structure%20%28by%20ref%29))
  (bind _cardlist (Variables|Default|GetCardList))
  ;[1 0 0.1556] Comment
  ;;[1 0 0.1556] Comment
  (if AddCardInList?
    (Utilities|Array|Add _cardlist Item)
    (else
      (Utilities|Array|RemoveItem _cardlist Item))))

(event Custom|S_AddPosture
  (params (BufferCaracPlayer :type ST%20Carac%20Player%202%20Structure))
  ;[1 0 0.1556] Comment
  ;;[1 0 0.1556] Comment
  (Variables|Default|SetBufferCaracPlayer (Utilities|Struct|MakeST_CaracPlayer2 (.Posture (Utilities|Struct|BreakST_CaracPlayer2 BufferCaracPlayer)) (.attaque (Variables|Default|GetBufferCaracPlayer)) (.defense (Variables|Default|GetBufferCaracPlayer)) (.vitesse (Variables|Default|GetBufferCaracPlayer)) (.pa (Variables|Default|GetBufferCaracPlayer)))))

(event Custom|S_AddbonusInfoEnnemy
  (params (BufferCaracPlayer :type ST%20Carac%20Player%202%20Structure))
  (bind (_posture _attaque _defense _vitesse) (Utilities|Struct|BreakST_CaracPlayer2 BufferCaracPlayer))
  ;[1 0 0.1556] Comment
  ;;[1 0 0.1556] Comment
  (Variables|Default|SetBonusEnnemyCarac (Utilities|Struct|MakeST_CaracPlayer2 "NewEnumerator3" (+ _attaque (.Attaque (Utilities|Struct|BreakST_CaracPlayer2 (Variables|Default|GetBonusEnnemyCarac)))) (+ _defense (.Defense (Utilities|Struct|BreakST_CaracPlayer2 (Variables|Default|GetBonusEnnemyCarac)))) (+ _vitesse (.Vitesse (Utilities|Struct|BreakST_CaracPlayer2 (Variables|Default|GetBonusEnnemyCarac)))) 0)))

(event Custom|S_AddRemovePA
  (params (BufferCaracPlayer :type ST%20Carac%20Player%202%20Structure) (AddPA? :type Boolean))
  (bind _pa (Utilities|Struct|BreakST_CaracPlayer2 BufferCaracPlayer))
  ;[1 0 0.1556] Comment
  ;;[1 0 0.1556] Comment
  (Variables|Default|SetBufferCaracPlayer (Utilities|Struct|MakeST_CaracPlayer2 (.Posture (Utilities|Struct|BreakST_CaracPlayer2 (Variables|Default|GetBufferCaracPlayer))) (.Attaque (Utilities|Struct|BreakST_CaracPlayer2 (Variables|Default|GetBufferCaracPlayer))) (.Defense (Utilities|Struct|BreakST_CaracPlayer2 (Variables|Default|GetBufferCaracPlayer))) (.Vitesse (Utilities|Struct|BreakST_CaracPlayer2 (Variables|Default|GetBufferCaracPlayer))) (select AddPA? (+ _pa (.PA (Utilities|Struct|BreakST_CaracPlayer2 (Variables|Default|GetBufferCaracPlayer)))) (- _pa (.PA (Utilities|Struct|BreakST_CaracPlayer2 (Variables|Default|GetBufferCaracPlayer))))))))

(event Custom|S_AddToBonusPlayer
  (params (BufferCaracPlayer :type ST%20Carac%20Player%202%20Structure))
  (bind (_posture _attaque _defense _vitesse) (Utilities|Struct|BreakST_CaracPlayer2 BufferCaracPlayer))
  ;[1 0 0.1556] Comment
  ;;[1 0 0.1556] Comment
  (Variables|Default|SetBonusPlayerCarac (Utilities|Struct|MakeST_CaracPlayer2 "NewEnumerator3" (+ _attaque (.Attaque (Utilities|Struct|BreakST_CaracPlayer2 (Variables|Default|GetBonusPlayerCarac)))) (+ _defense (.Defense (Utilities|Struct|BreakST_CaracPlayer2 (Variables|Default|GetBonusPlayerCarac)))) (+ _vitesse (.Vitesse (Utilities|Struct|BreakST_CaracPlayer2 (Variables|Default|GetBonusPlayerCarac)))) 0)))

(fn ConstructionScript)

(fn PCKlaftGameAutoGenFunc
  (params (ActivePlayerIndex :type Integer))
  (bind _asbp_character (Utilities|Casting|CastToBP_Character (Pawn|GetControlledPawn self)))
  (Variables|/Game/CoreKlaft/BP_Character.BP_Character_C|SetPlayerInfoCurrentGame _asbp_character (Variables|/Game/CoreKlaft/BP_Character.BP_Character_C|GetRefInfoPlayer _asbp_character))
  (if (== ActivePlayerIndex (Variables|Default|GetIndexPlayer))
    (Variables|Default|SetIsMyTurn? true)
    (else
      (Variables|Default|SetIsMyTurn? false))))

(fn GetHitTilefromCursor
  (bind _hitresult (Game|Player|GetHitResultUnderCursorbyChannel "TraceTypeQuery1" true))
  (bind (_bblockinghit _binitialoverlap _time _distance _location _impactpoint _normal _impactnormal _physmat _hitactor) (Collision|BreakHitResult _hitresult))
  (bind _asbp_tile_contener_grid (Utilities|Casting|CastToBP_TileContenerGrid (Actor|GetParentActor _hitactor))
    (:then
      (return _location _asbp_tile_contener_grid))
    (:CastFailed
      (return "0, 0, 0" 0))))

(fn GetPlayerPawn
  (bind _asbp_character (Utilities|Casting|CastToBP_Character (Pawn|GetControlledPawn)))
  (return _asbp_character))

(fn ResolutionBonusPosture
  (params (CaracPlayer :type ST%20Carac%20Player%202%20Structure) (CaracPlayer2 :type ST%20Carac%20Player%202%20Structure))
  (bind _valuebonusposture (Variables|Default|GetValueBonusPosture))
  (bind _valuebonusposture_2 (Variables|Default|GetValueBonusPosture))
  (Utilities|FlowControl|Sequence
    (:then_0
      ;[1 1 1] Player
      (bind _output_get (LocalVariables|SetL_CaracPlayer1 CaracPlayer))
      (LocalVariables|SetL_CaracPlayer1 (Utilities|Struct|MakeST_CaracPlayer2 (.posture (LocalVariables|GetL_CaracPlayer1)) (Utilities|Select :Index (.posture _output_get) :NewEnumerator3 0 :NewEnumerator1 (+ (.attaque _output_get) _valuebonusposture) :NewEnumerator0 (.attaque _output_get) :NewEnumerator2 (.attaque _output_get)) (Utilities|Select :Index (.posture _output_get) :NewEnumerator3 0 :NewEnumerator1 (.defense _output_get) :NewEnumerator0 (+ (.defense _output_get) _valuebonusposture) :NewEnumerator2 (.defense _output_get)) (Utilities|Select :Index (.posture _output_get) :NewEnumerator3 0 :NewEnumerator1 (.vitesse _output_get) :NewEnumerator0 (.vitesse _output_get) :NewEnumerator2 (+ (.vitesse _output_get) _valuebonusposture)) (.pa (LocalVariables|GetL_CaracPlayer1)))))
    (:then_1
      ;[1 1 1] Player2
      (bind _output_get_2 (LocalVariables|SetL_CaracPlayer2 CaracPlayer2))
      (LocalVariables|SetL_CaracPlayer2 (Utilities|Struct|MakeST_CaracPlayer2 (.posture (LocalVariables|GetL_CaracPlayer2)) (Utilities|Select :Index (.posture _output_get_2) :NewEnumerator3 0 :NewEnumerator1 (+ (.attaque _output_get_2) _valuebonusposture_2) :NewEnumerator0 (.attaque _output_get_2) :NewEnumerator2 (.attaque _output_get_2)) (Utilities|Select :Index (.posture _output_get_2) :NewEnumerator3 0 :NewEnumerator1 (.defense _output_get_2) :NewEnumerator0 (+ (.defense _output_get_2) _valuebonusposture_2) :NewEnumerator2 (.defense _output_get_2)) (Utilities|Select :Index (.posture _output_get_2) :NewEnumerator3 0 :NewEnumerator1 (.vitesse _output_get_2) :NewEnumerator0 (.vitesse _output_get_2) :NewEnumerator2 (+ (.vitesse _output_get_2) _valuebonusposture_2)) (.pa (LocalVariables|GetL_CaracPlayer2)))))
    (:then_3
      (return (LocalVariables|GetL_CaracPlayer1) (LocalVariables|GetL_CaracPlayer2)))))

(fn ResolutionCaracFight
  (params (CaracPlayer :type ST%20Carac%20Player%202%20Structure) (CaracPlayer2 :type ST%20Carac%20Player%202%20Structure))
  (LocalVariables|SetL_Player CaracPlayer)
  (LocalVariables|SetL_Player2 CaracPlayer2)
  (Utilities|FlowControl|Sequence
    (:then_0
      ;[1 1 1] Comment
      (LocalVariables|SetL_VitessePlayer (.Vitesse (Utilities|Struct|BreakST_CaracPlayer2 (LocalVariables|GetL_Player))))
      (LocalVariables|SetL_VitessePlayer2 (.Vitesse (Utilities|Struct|BreakST_CaracPlayer2 (LocalVariables|GetL_Player2)))))
    (:then_1
      ;[1 1 1] Comment
      (Math|Integer|CompareInt (.Vitesse (Utilities|Struct|BreakST_CaracPlayer2 (LocalVariables|GetL_Player))) (.Defense (Utilities|Struct|BreakST_CaracPlayer2 (LocalVariables|GetL_Player2)))
        (:>
          (LocalVariables|SetL_VitessePlayer (+ (LocalVariables|GetL_VitessePlayer) (.Vitesse (Utilities|Struct|BreakST_CaracPlayer2 (LocalVariables|GetL_Player))))))
        (:==)
        (:<
          (LocalVariables|SetL_VitessePlayer2 (+ (LocalVariables|GetL_VitessePlayer2) (.Defense (Utilities|Struct|BreakST_CaracPlayer2 (LocalVariables|GetL_Player2))))))))
    (:then_2
      ;[1 1 1] Comment
      (Math|Integer|CompareInt (.Defense (Utilities|Struct|BreakST_CaracPlayer2 (LocalVariables|GetL_Player))) (.Attaque (Utilities|Struct|BreakST_CaracPlayer2 (LocalVariables|GetL_Player2)))
        (:>
          (LocalVariables|SetL_VitessePlayer (+ (LocalVariables|GetL_VitessePlayer) (.Defense (Utilities|Struct|BreakST_CaracPlayer2 (LocalVariables|GetL_Player))))))
        (:==)
        (:<
          (LocalVariables|SetL_VitessePlayer2 (+ (LocalVariables|GetL_VitessePlayer2) (.Attaque (Utilities|Struct|BreakST_CaracPlayer2 (LocalVariables|GetL_Player2))))))))
    (:then_3
      (return (LocalVariables|GetL_VitessePlayer) (LocalVariables|GetL_VitessePlayer2)))))

(fn ResolutionBonusCard
  (params (CaracPlayer :type ST%20Carac%20Player%202%20Structure) (CaracPlayer2 :type ST%20Carac%20Player%202%20Structure) (BonusPlayer1 :type ST%20Carac%20Player%202%20Structure) (Bonus%20Player2 :type ST%20Carac%20Player%202%20Structure))
  (LocalVariables|SetL_CaractPlayer1 CaracPlayer)
  (LocalVariables|SetL_CaractPlayer2 CaracPlayer2)
  (LocalVariables|SetL_BonusPlayer1 BonusPlayer1)
  (LocalVariables|SetL_BonusPlayer2 Bonus%20Player2)
  (LocalVariables|SetL_CaractPlayer1 (Utilities|Struct|MakeST_CaracPlayer2 (.posture (LocalVariables|GetL_CaractPlayer1)) (+ (.attaque (LocalVariables|GetL_CaractPlayer1)) (.attaque (LocalVariables|GetL_BonusPlayer1))) (+ (.defense (LocalVariables|GetL_CaractPlayer1)) (.defense (LocalVariables|GetL_BonusPlayer1))) (+ (.vitesse (LocalVariables|GetL_CaractPlayer1)) (.vitesse (LocalVariables|GetL_BonusPlayer1))) (.pa (LocalVariables|GetL_CaractPlayer1))))
  (LocalVariables|SetL_CaractPlayer2 (Utilities|Struct|MakeST_CaracPlayer2 (.posture (LocalVariables|GetL_CaractPlayer2)) (+ (.attaque (LocalVariables|GetL_CaractPlayer2)) (.attaque (LocalVariables|GetL_BonusPlayer2))) (+ (.defense (LocalVariables|GetL_CaractPlayer2)) (.defense (LocalVariables|GetL_BonusPlayer2))) (+ (.vitesse (LocalVariables|GetL_CaractPlayer2)) (.vitesse (LocalVariables|GetL_BonusPlayer2))) (.pa (LocalVariables|GetL_CaractPlayer2))))
  (return (LocalVariables|GetL_CaractPlayer1) (LocalVariables|GetL_CaractPlayer2)))

(fn ResolutionBonusCoruption
  (params (CaracPlayer :type ST%20Carac%20Player%202%20Structure) (CaracPlayer2 :type ST%20Carac%20Player%202%20Structure))
  (return CaracPlayer CaracPlayer2))

(fn NewFunction0
  (params (CaracPlayer :type ST%20Carac%20Player%202%20Structure) (CaracPlayer2 :type ST%20Carac%20Player%202%20Structure) (BonusPlayer1 :type ST%20Carac%20Player%202%20Structure) (Bonus%20Player2 :type ST%20Carac%20Player%202%20Structure))
  (bind (_newcaracplayer _newcaracplayer2) (CallFunction|ResolutionBonusPosture CaracPlayer CaracPlayer2))
  (bind (_newcaracplayer_2 _newcaracplayer2_2) (CallFunction|ResolutionBonusCard _newcaracplayer _newcaracplayer2 BonusPlayer1 Bonus%20Player2))
  (bind (_l_vitesseplayer1 _l_vitesseplayer21) (CallFunction|ResolutionCaracFight _newcaracplayer_2 _newcaracplayer2_2))
  (return _l_vitesseplayer1 _l_vitesseplayer21))

(fn PAModule)

(fn OnRepCardList)

(fn OnRepNbGemme)

(fn OnRepBufferCaracEnnemy)

(fn OnRepBonusPlayerCarac)

(fn OnRepBonusEnnemyCarac)

(fn OnRepCardMaxHand)

(fn FoundPlayerController
  (params (IndexPlayer :type Integer))
  (LocalVariables|SetNewLocalVar_0 false)
  (bind _array_element (Utilities|Array|ForEachLoopwithBreak (Variables|/Game/CoreKlaft/GM_KlaftGame.GM_KlaftGame_C|GetListPlayer (.AsGM%20Klaft%20Game (Utilities|Casting|CastToGM_KlaftGame (Game|GetGameMode)))) :!label _label)
    (:LoopBody
      (LocalVariables|SetNewLocalVar_1 (.AsPC%20Klaft%20Game (Utilities|Casting|CastToPC_KlaftGame _array_element)))
      (if (== (Variables|PC_KlaftGame_C|GetIndexPlayer (.AsPC%20Klaft%20Game (Utilities|Casting|CastToPC_KlaftGame _array_element))) IndexPlayer)
        (Utilities|FlowControl|Sequence
          (:then_0
            (LocalVariables|SetNewLocalVar_0 true))
          (:then_1
            (goto _label Break)))))
    (:Completed
      (if (LocalVariables|GetNewLocalVar_0)
        (return (LocalVariables|GetNewLocalVar_1))
        (else
          (return 0))))))