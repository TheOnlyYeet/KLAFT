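; Game mode for Klaft, a three-player turn-based game with movement on tiles.
; On login or controller swap, a count of three players triggers a delayed setup that indexes and lists the controllers, then has GMS_Klaft begin the first turn.
; RespawnCharacter replaces a pawn at an untagged PlayerStart, tagging it as used.
; Helper functions rotate the active turn and move the character to a nearby tile under the cursor.
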(event EventPostLogin
  (params (NewPlayer :type Player%20Controller%20Object%20Reference))
  (bind _returnvalue (Class|GameModeBase|GetNumPlayers))
  (if (== _returnvalue 3)
    (Development|PrintString "DELAY")
    (Utilities|FlowControl|Delay 3.0)
    (Utilities|FlowControl|Sequence
      (:then_0
        (Default|CSetPlayerIndex (Utilities|GetPlayerController))
        (Default|CSetPlayerIndex (Utilities|GetPlayerController 1) 1)
        (Default|CSetPlayerIndex (Utilities|GetPlayerController 2) 2))
      (:then_1
        (Utilities|Array|Add (Variables|Default|GetListPlayer) (Utilities|GetPlayerController))
        (Utilities|Array|Add (Variables|Default|GetListPlayer) (Utilities|GetPlayerController 1))
        (Utilities|Array|Add (Variables|Default|GetListPlayer) (Utilities|GetPlayerController 2)))
      (:then_2
        (Default|MBeginPlayerTurn (.AsGMS%20Klaft (Utilities|Casting|CastToGMS_Klaft (Game|GetGameState))))))))

(event EventOnSwapPlayerControllers
  (params (OldPC :type Player%20Controller%20Object%20Reference) (NewPC :type Player%20Controller%20Object%20Reference))
  (bind _returnvalue (Class|GameModeBase|GetNumPlayers))
  (if (== _returnvalue 3)
    (Development|PrintString "DELAY")
    (Utilities|FlowControl|Delay 3.0)
    (Utilities|FlowControl|Sequence
      (:then_0
        (Default|CSetPlayerIndex (Utilities|GetPlayerController))
        (Default|CSetPlayerIndex (Utilities|GetPlayerController 1) 1)
        (Default|CSetPlayerIndex (Utilities|GetPlayerController 2) 2))
      (:then_1
        (Utilities|Array|Add (Variables|Default|GetListPlayer) (Utilities|GetPlayerController))
        (Utilities|Array|Add (Variables|Default|GetListPlayer) (Utilities|GetPlayerController 1))
        (Utilities|Array|Add (Variables|Default|GetListPlayer) (Utilities|GetPlayerController 2)))
      (:then_2
        (Default|MBeginPlayerTurn (.AsGMS%20Klaft (Utilities|Casting|CastToGMS_Klaft (Game|GetGameState))))))))

(event Custom|RespawnCharacter
  (params (InputPin :type Actor%20Class%20Reference) (Target :type Controller%20Object%20Reference))
  (bind _returnvalue (Pawn|GetControlledPawn Target))
  (Utilities|IsValid _returnvalue
    (:Is%20Valid
      (Actor|DestroyActor _returnvalue))
    (:Is%20Not%20Valid
      _))
  (bind _outactors (Actor|GetAllActorsOfClass "/Script/Engine.PlayerStart"))
  (bind _array_element (Utilities|Array|ForEachLoopwithBreak _outactors :!label _label)
    (:LoopBody
      (if (Utilities|Name|NotEqual(Name) (Variables|/Script/Engine.PlayerStart|GetPlayerStartTag _array_element) "Found")
        (Variables|/Script/Engine.PlayerStart|SetPlayerStartTag _array_element "Found")
        (goto _label Break)))
    (:Completed
      (Game|SpawnActorfromClass InputPin (Math|Transform|MakeTransform (.location (Transformation|GetActorTransform _array_element)) (.rotation (Transformation|GetActorTransform _array_element)) "1,1,1") "AlwaysSpawn" 0 0)
      (Pawn|Possess Target))))

(fn ConstructionScript)

(fn InitializationNewIndexPlayer
  (Variables|/Game/CoreKlaft/PC_KlaftGame.PC_KlaftGame_C|SetIsMyTurn? (.AsPC%20Klaft%20Game (Utilities|Casting|CastToPC_KlaftGame (Utilities|Array|Get(acopy) (Variables|Default|GetOrder) (Variables|Default|GetIndexControllerIsPlay)))) false)
  ;[1 1 1] NextIndexPlayer
  (if (== (Variables|Default|GetIndexControllerIsPlay) 2)
    (Variables|Default|SetIndexControllerIsPlay 0)
    (else
      (Variables|Default|SetIndexControllerIsPlay (+ (Variables|Default|GetIndexControllerIsPlay) 1))))
  (Variables|/Game/CoreKlaft/PC_KlaftGame.PC_KlaftGame_C|SetIsMyTurn? (.AsPC%20Klaft%20Game (Utilities|Casting|CastToPC_KlaftGame (Utilities|Array|Get(acopy) (Variables|Default|GetOrder) (Variables|Default|GetIndexControllerIsPlay)))) true))

(fn MoveAction
  (bind _refcontrollerisplayed (Variables|Default|GetRefControllerIsPlayed))
  (bind _hitresult (Game|Player|GetHitResultUnderCursorbyChannel _refcontrollerisplayed "TraceTypeQuery1" true))
  (bind _asbp_character (Utilities|Casting|CastToBP_Character (Pawn|GetControlledPawn (Variables|Default|GetRefControllerIsPlayed))))
  (if (not (Variables|/Game/CoreKlaft/BP_Character.BP_Character_C|GetPawnMoving? _asbp_character))
    (bind _asbp_tileversoin_2 (Utilities|Casting|CastToBP_Tileversoin2 (.hitactor _hitresult)))
    (if (<= (Math|Vector|Distance(Vector) (.location _hitresult) (Transformation|GetActorLocation _asbp_character)) 2e+02)
      (Default|SMovingInializationAction _asbp_character (Transformation|GetActorLocation _asbp_tileversoin_2)))))

(fn OnRepIndexControllerIsPlay)

(fn OnRepListPlayer)

(fn GetPlayerInfo
  (params (IndexPlayer :type Integer))
  (bind _aspc_klaft_game (Utilities|Casting|CastToPC_KlaftGame (Utilities|Array|Get(acopy) (Variables|Default|GetListPlayer) IndexPlayer)))
  (return _aspc_klaft_game))