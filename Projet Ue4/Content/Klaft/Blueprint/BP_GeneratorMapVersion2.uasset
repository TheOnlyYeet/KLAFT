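; Procedural hex board generator that lays out regions, transition borders, a start row and a tapering boss zone.
; NewMacro0 builds a colored static mesh preview, stepping height per region, and assigns seeded random terrain into TestInfoGenerationBaseBoard, keyed by location.
; Reconstruction removes the preview and spawns rotated BP_TileContenerGrid actors from that data, plus PlayerStarts on start tiles.
; Clear destroys the spawned tiles.
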(event Custom|Reconstruction
  (bind _testinfogenerationbaseboard (Variables|Default|GetTestInfoGenerationBaseBoard))
  (Utilities|Clearin
    (:Completed
      (bind _outactors (Actor|GetAllActorsOfClass "BP_GeneratorMapVersion2_C"))
      (Variables|Default|SetNewVar_1 (Transformation|GetActorRotation (Utilities|Array|Get(acopy) _outactors)))
      (bind _keys (Utilities|Map|Keys (.map _testinfogenerationbaseboard)))
      (for _array_element _keys
        (bind _returnvalue (Game|SpawnActorfromClass "/Game/Klaft/Blueprint/BP_TileContenerGrid.BP_TileContenerGrid_C" (Math|Transform|MakeTransform (Math|Vector|RotateVector (+ _array_element (Transformation|GetActorLocation)) (Variables|Default|GetNewVar_1)) (Variables|Default|GetNewVar_1) "1,1,1") "Undefined" 0 (.Value (Utilities|Map|Find (.map _testinfogenerationbaseboard) _array_element)) (Utilities|Map|Contains (.transitionmapindexregion _testinfogenerationbaseboard) _array_element) "NewEnumerator0" (.Value (Utilities|Map|Find (Variables|Default|GetGridZone) _array_element)) "NewEnumerator0" "NewEnumerator0" "NewEnumerator0" 0))
        (Utilities|Array|Add (Variables|Default|GetTileSpawned) _returnvalue))
      (bind _keys_2 (Utilities|Map|Keys (.boss _testinfogenerationbaseboard)))
      (for _array_element_2 _keys_2
        (bind _returnvalue_2 (Game|SpawnActorfromClass "/Game/Klaft/Blueprint/BP_TileContenerGrid.BP_TileContenerGrid_C" (Math|Transform|MakeTransform (Math|Vector|RotateVector (+ _array_element_2 (Transformation|GetActorLocation)) (Variables|Default|GetNewVar_1)) (Variables|Default|GetNewVar_1) "1,1,1") "Undefined" 0 (.Value (Utilities|Map|Find (.boss _testinfogenerationbaseboard) _array_element_2)) false "NewEnumerator0" (.Value (Utilities|Map|Find (Variables|Default|GetGridZone) _array_element_2)) "NewEnumerator0" "NewEnumerator0" "NewEnumerator0" 0))
        (Utilities|Array|Add (Variables|Default|GetTileSpawned) _returnvalue_2))
      (bind _keys_3 (Utilities|Map|Keys (.start _testinfogenerationbaseboard)))
      (for _array_element_3 _keys_3
        (bind _returnvalue_3 (Game|SpawnActorfromClass "/Game/Klaft/Blueprint/BP_TileContenerGrid.BP_TileContenerGrid_C" (Math|Transform|MakeTransform (Math|Vector|RotateVector (+ _array_element_3 (Transformation|GetActorLocation)) (Variables|Default|GetNewVar_1)) (Variables|Default|GetNewVar_1) "1,1,1") "Undefined" 0 (.Value (Utilities|Map|Find (.start _testinfogenerationbaseboard) _array_element_3)) false "NewEnumerator0" (.Value (Utilities|Map|Find (Variables|Default|GetGridZone) _array_element_3)) "NewEnumerator0" "NewEnumerator0" "NewEnumerator0" 0))
        (Utilities|Array|Add (Variables|Default|GetTileSpawned) _returnvalue_3)
        (Game|SpawnActorfromClass "/Script/Engine.PlayerStart" (Math|Transform|MakeTransform (+ (Math|Vector|RotateVector (+ _array_element_3 (Transformation|GetActorLocation)) (Variables|Default|GetNewVar_1)) "0, 0,90.000000") (Math|Rotator|CombineRotators (Variables|Default|GetNewVar_1) "0,90.000000, 0") "1,1,1") "Undefined" 0 0)))))

(event Custom|Clear
  (bind _tilespawned (Variables|Default|GetTileSpawned))
  (for _array_element _tilespawned
    (Actor|DestroyActor _array_element))
  (Utilities|Array|Clear _tilespawned))

(event Custom|ConstructionScript
  (Utilities|NewMacro0))

(fn ConstructionScript)

(fn IndexforCreateX
  (return (- (* (Variables|Default|GetSizeBorder) -1) 1) (- (+ (Variables|Default|GetGridSizeX) (Variables|Default|GetSizeBorder)) 1)))

(fn IndexforCreateY
  (params (A :type Integer))
  (return (- (* (Variables|Default|GetSizeBorder) -1) 1) (- (+ A (Variables|Default|GetSizeBorder)) 1)))

(fn CalculLocatioGridHexa
  (params (CurrentIndexY :type Integer) (CurrentIndexX :type Integer))
  (bind _returnvalue (Math|Integer|%(Integer) CurrentIndexX 2))
  (bind _spacingx (Variables|Default|GetSpacingX))
  (bind _spacingy (Variables|Default|GetSpacingY))
  (bind _returnvalue_2 (== _returnvalue 0))
  (bind _returnvalue_3 (* CurrentIndexY _spacingy))
  (bind _returnvalue_4 (* CurrentIndexX _spacingx))
  (return (Math|Vector|SelectVector (Math|Vector|MakeVector _returnvalue_4 _returnvalue_3 0.0) (Math|Vector|MakeVector _returnvalue_4 (+ _returnvalue_3 (Variables|Default|GetOffset)) 0.0) (not _returnvalue_2)) _returnvalue_2))