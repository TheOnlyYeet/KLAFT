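; Player character Blueprint for a networked game that moves to a target point by turning toward it, then gliding there.
; A server-named event forwards the target to a multicast-named event, which ignores new requests while moving.
; Two chained timelines lerp yaw, then XY position at fixed height, with play rates set from duration variables at BeginPlay.
; Debug prints and a NumPad 0 test of replicated upward offsets remain.
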(event Custom|S_Test
  (Transformation|AddActorLocalOffset "0, 0,500.000000" false false))

(event Custom|C_Test
  (Transformation|AddActorLocalOffset "0, 0,500.000000" false false))

(event Custom|M_Test
  (Transformation|AddActorLocalOffset "0, 0,500.000000" false false))

(event EventBeginPlay
  (CallFunction|SetupTimeAnim))

(event Input|KeyboardEvents|NumPadZero
  (params (Key :type Key%20Structure :default "None"))
  (:Pressed
    (Networking|SwitchHasAuthority
      (:Authority
        (CallFunction|STest))
      (:Remote
        (CallFunction|STest)
        (CallFunction|CTest)))))

(event Custom|S_MovingInializationAction
  (params (NewParam :type Vector))
  (CallFunction|MMovingPawn NewParam)
  (Development|PrintString "gggg" true true "(R=0.000000,G=0.056146,B=0.085069,A=1.000000)"))

(event Custom|M_MovingPawn
  (params (LoctionPlayerTarget :type Vector))
  (Development|PrintString "gggg" true true "(R=0.085069,G=0.000000,B=0.004348,A=1.000000)")
  (if (not (Variables|Default|GetPawnMoving?))
    (Variables|Default|SetPawnMoving? true)
    (Variables|Default|SetLoctionPlayerTarget LoctionPlayerTarget)
    (Variables|Default|SetLocationPlayerStart (Transformation|GetActorLocation))
    (Variables|Default|SetRotationCameraStart (Transformation|GetActorRotation))
    ;[1 1 1] Step 1 : Rotation Pawn
    (bind _percentanim (Timeline|AnimRotate PlayFromStart)
      (:Update
        (CallFunction|SetrotationPawn _percentanim))
      (:Finished
        ;[1 1 1] Step 2 : Move pawn
        (bind _percentanim_2 (Timeline|AnimMove PlayFromStart)
          (:Update
            (CallFunction|SetLocationPawn _percentanim_2))
          (:Finished
            (Variables|Default|SetPawnMoving? false)))))))

(fn ConstructionScript)

(fn SetLocationPawn
  (params (Alpha :type Float%20%28single-precision%29))
  (bind _loctionplayertarget (Variables|Default|GetLoctionPlayerTarget))
  (bind (_x _y) (Math|Vector|BreakVector _loctionplayertarget))
  (Transformation|SetActorLocation (Math|Vector|Lerp(Vector) (Variables|Default|GetLocationPlayerStart) (Math|Vector|MakeVector _x _y (.Z (Math|Vector|BreakVector (Variables|Default|GetLocationPlayerStart)))) Alpha) false false))

(fn SetrotationPawn
  (params (Alpha :type Float%20%28single-precision%29))
  (bind _rotationcamerastart (Variables|Default|GetRotationCameraStart))
  (Transformation|SetActorRotation (Math|Rotator|Lerp(Rotator) (Variables|Default|GetRotationCameraStart) (Math|Rotator|MakeRotator (.roll _rotationcamerastart) (.pitch _rotationcamerastart) (.yaw (Math|Rotator|FindLookatRotation (Variables|Default|GetLocationPlayerStart) (Variables|Default|GetLoctionPlayerTarget)))) Alpha true)))

(fn SetupTimeAnim
  (Components|Timeline|SetPlayRate (Variables|Default|GetAnimRotate) (/ 1.0 (Variables|Default|GetDurationAnimRotate)))
  (Components|Timeline|SetPlayRate (Variables|Default|GetAnimMove) (/ 1.0 (Variables|Default|GetDurationAnimMove))))