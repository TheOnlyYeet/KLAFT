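; BP_TileContenerGrid is a two-sided grid tile that can flip over and trigger an enemy fight.
; Construction builds back-to-back BP_Tileversoin2 child actors on a pivot, sets movement flags by tile type, and reruns from BeginPlay on authority via server/multicast-named events.
; S_InitializeAnimTile plays a 180-degree timeline flip, guarded against re-entry.
; On finish, enemy tiles spawn BP_CharacterEnemy facing the player's pawn, then start the controller's fight module after a delay.
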(event Custom|S_SpawnEnemy
  (params (PC :type PC%20Klaft%20Game%20Object%20Reference))
  (bind _returnvalue (Game|SpawnActorfromClass "/Game/CoreKlaft/BP_CharacterEnemy.BP_CharacterEnemy_C" (Math|Conversions|ToTransform(Vector) (+ (Transformation|GetActorLocation) "0, 0,96.000000")) "Undefined" 0 0))
  (bind _output_get (Variables|Default|SetRefEnemyPawn _returnvalue))
  (Default|SRotateEnemy _output_get (Transformation|GetActorLocation (Pawn|GetControlledPawn PC)))
  (Utilities|FlowControl|Delay 2.0)
  (Default|SFightSystemModule PC (Variables|Default|GetRefEnemyPawn) self))

(event Custom|S_InitializeAnimTile
  (params (PC :type PC%20Klaft%20Game%20Object%20Reference))
  (if (not (Variables|Default|GetAnimationIsPlaying?))
    (Variables|Default|SetAnimationIsPlaying? true)
    (Variables|Default|SetRelative%20Rotation (Transformation|GetActorRotation))
    (Utilities|FlowControl|FlipFlop
      (:A
        (bind _percentanimation (Timeline|Animation PlayFromStart)
          (:Update
            (Transformation|SetActorRotation (Math|Rotator|Lerp(Rotator) (Variables|Default|GetRelative%20Rotation) (Math|Rotator|CombineRotators (Variables|Default|GetRelative%20Rotation) "180.000000, 0, 0") _percentanimation true)))
          (:Finished
            (Variables|Default|SetRelative%20Rotation (Transformation|GetActorRotation))
            (Variables|Default|SetAnimationIsPlaying? false)
            (if (Variables|Default|GetEnemy?)
              (CallFunction|SSpawnEnemy PC)))))
      (:B
        (Timeline|Animation PlayFromStart)))))

(event Custom|M_Construction
  (if (Variables|SettingsBaseTile|GetTransitionTile?)
    (Variables|Default|SetIndexTransition (+ (Variables|SettingsBaseTile|GetRegionIndex) 1)))
  (Utilities|ConstructionStr))

(event Custom|S_ConstructionScript
  (CallFunction|MConstruction))

(event EventBeginPlay
  (Components|Timeline|SetPlayRate (Variables|Default|GetAnimation) (/ 1.0 (Variables|SettingsBaseTile|GetDurationAnimation)))
  (Networking|SwitchHasAuthority
    (:Authority
      (CallFunction|SConstructionScript))))

(fn ConstructionScript
  (if (Variables|SettingsBaseTile|GetTransitionTile?)
    (Variables|Default|SetIndexTransition (+ (Variables|SettingsBaseTile|GetRegionIndex) 1)))
  (Utilities|ConstructionStr))

(fn SetupConstruction
  (Default|SetupTile (.AsBP%20Tileversoin%202 (Utilities|Casting|CastToBP_Tileversoin2 (Variables|/Script/Engine.ChildActorComponent|GetChildActor (Variables|Default|GetTile2)))) (Variables|SettingsT2|GetTypeTile_2))
  (Default|SetupTile (.AsBP%20Tileversoin%202 (Utilities|Casting|CastToBP_Tileversoin2 (Variables|/Script/Engine.ChildActorComponent|GetChildActor (Variables|Default|GetTile1)))) (Variables|SettingsT1|GetTypeTile)))

(fn OnRepRefEnemyPawn)