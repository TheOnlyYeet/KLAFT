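; Turn-based player character that spends action points (PA) to move and ends its turn when none remain.
; BeginPlay copies player stats with a random PA bonus, then spawns a separate BP_Camera as the controller's view target.
; S_Moving deducts a point and passes the target through S_/M_ events, where chained timelines turn the pawn toward it, then slide it there at constant height.
; The OnRep handlers are empty.
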(event Custom|CreateCameraPlayer
  (bind _socketcamera (Variables|Default|GetSocketCamera))
  (bind _returnvalue (Transformation|GetWorldTransform _socketcamera))
  (bind _returnvalue_2 (Game|SpawnActorfromClass "/Game/CoreKlaft/BP_Camera.BP_Camera_C" (Math|Transform|MakeTransform (.location _returnvalue) (Math|Rotator|MakeRotator 0.0 0.0 (.Yaw (Math|Rotator|BreakRotator (.rotation _returnvalue)))) "1,1,1") "Undefined" 0 0))
  (bind _output_get (Variables|Default|SetRefCamera _returnvalue_2))
  (Transformation|SetWorldRotation (Variables|/Game/CoreKlaft/BP_Camera.BP_Camera_C|GetCamera _output_get) (.rotation _returnvalue) false false)
  (Game|Player|SetViewTargetwithBlend (.AsPC%20Klaft%20Game (Utilities|Casting|CastToPC_KlaftGame (Pawn|GetController self))) _output_get 0.0 "VTBlend_Linear" 0.0 false))

(event Custom|S_Moving
  (params (NewParam :type Vector))
  ;[0 0.8887 1] Pa Module
  (if (> (.pa (Variables|Default|GetPlayerInfoCurrentGame)) 0)
    (if (== (- (.pa (Variables|Default|GetPlayerInfoCurrentGame)) 1) 0)
      (Variables|Default|SetIsMyTour? false))
    (Variables|Default|SetPlayerInfoCurrentGame (Utilities|Struct|MakeST_CaracPlayer2 (.posture (Variables|Default|GetPlayerInfoCurrentGame)) (.attaque (Variables|Default|GetPlayerInfoCurrentGame)) (.defense (Variables|Default|GetPlayerInfoCurrentGame)) (.vitesse (Variables|Default|GetPlayerInfoCurrentGame)) (- (.pa (Variables|Default|GetPlayerInfoCurrentGame)) 1)))
    (CallFunction|SMovingInializationAction NewParam)
    (else
      (Variables|Default|SetIsMyTour? false))))

(event Custom|S_IniatilisationTour
  (bind _refinfoplayer (Variables|Default|GetRefInfoPlayer))
  (Variables|Default|SetPlayerInfoCurrentGame (Utilities|Struct|MakeST_CaracPlayer2 (.posture _refinfoplayer) (.attaque _refinfoplayer) (.defense _refinfoplayer) (.vitesse _refinfoplayer) (+ (.pa _refinfoplayer) (Variables|Default|GetRandomPaValue)))))

(event EventBeginPlay
  (Variables|Default|SetRandomPaValue (Math|Random|RandomIntegerinRange 1 5))
  (CallFunction|SIniatilisationTour)
  (CallFunction|CreateCameraPlayer))

(event Custom|S_MovingInializationAction
  (params (NewParam :type Vector))
  (CallFunction|MMovingPawn NewParam))

(event Custom|M_MovingPawn
  (params (LoctionPlayerTarget :type Vector))
  (if (not (Variables|Default|GetPawnMoving?))
    (Variables|Default|SetPawnMoving? true)
    (Variables|Default|SetLoctionPlayerTarget LoctionPlayerTarget)
    (Variables|Default|SetLocationPlayerStart (Transformation|GetActorLocation))
    (Variables|Default|SetRotationCameraStart (Transformation|GetActorRotation))
    ;[1 1 1] Step 1 : Rotation Pawn
    (bind _percentanim (Timeline|AnimRotate PlayFromStart)
      (:Update
        (CallFunction|SetrotationPawn _percentanim))
      (:Finished
        ;[1 1 1] Step 2 : Move pawn
        (bind _percentanim_2 (Timeline|AnimMove PlayFromStart)
          (:Update
            (CallFunction|SetLocationPawn _percentanim_2))
          (:Finished
            (Variables|Default|SetPawnMoving? false)))))))

(fn ConstructionScript)

(fn SetLocationPawn
  (params (Alpha :type Float%20%28single-precision%29))
  (bind _loctionplayertarget (Variables|Default|GetLoctionPlayerTarget))
  (bind (_x _y) (Math|Vector|BreakVector _loctionplayertarget))
  (Transformation|SetActorLocation (Math|Vector|Lerp(Vector) (Variables|Default|GetLocationPlayerStart) (Math|Vector|MakeVector _x _y (.Z (Math|Vector|BreakVector (Variables|Default|GetLocationPlayerStart)))) Alpha) false false))

(fn SetrotationPawn
  (params (Alpha :type Float%20%28single-precision%29))
  (bind _rotationcamerastart (Variables|Default|GetRotationCameraStart))
  (Transformation|SetActorRotation (Math|Rotator|Lerp(Rotator) (Variables|Default|GetRotationCameraStart) (Math|Rotator|MakeRotator (.roll _rotationcamerastart) (.pitch _rotationcamerastart) (.yaw (Math|Rotator|FindLookatRotation (Variables|Default|GetLocationPlayerStart) (Variables|Default|GetLoctionPlayerTarget)))) Alpha true)))

(fn SetupTimeAnim
  (Components|Timeline|SetPlayRate (Variables|Default|GetAnimRotate) (/ 1.0 (Variables|Default|GetDurationAnimRotate)))
  (Components|Timeline|SetPlayRate (Variables|Default|GetAnimMove) (/ 1.0 (Variables|Default|GetDurationAnimMove))))

(fn OnRepInfoPlayer)

(fn OnRepPlayerInfoCurrentGame)

(fn OnRepIsMyTour?)

(fn OnRepNewVar0)

(fn OnRepSateANim)