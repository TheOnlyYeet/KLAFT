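; Player controller for a networked, turn-based tile game, spawning the selected character at an untagged PlayerStart and possessing it.
; The game state's active player index sets IsMyTurn, gating clicks that animate movable tiles within range of the pawn.
; Server-prefixed events handle movement, action-point decrements, turn end and player-versus-enemy fights.
; The ModuleFight macro chains posture bonuses, card bonuses and stat comparison into Win, Equal or Lose; the corruption bonus is an unused pass-through.
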(event Custom|S_RespawnCharacter
  (bind _asbp_pmm_instance (Utilities|Casting|CastToBP_PMM_Instance (Game|GetGameInstance)))
  (Default|RespawnCharacter (.AsGM%20Klaft%20Game (Utilities|Casting|CastToGM_KlaftGame (Game|GetGameMode))) (Variables|/Game/CoreKlaft/BP_PMM_Instance.BP_PMM_Instance_C|GetCharacterSelection _asbp_pmm_instance) self))

(event Custom|C_SpawnCharacter
  (params (Controller :type Controller%20Object%20Reference))
  (Development|PrintString "SpawnPlayer" true true "(R=0.207907,G=1.000000,B=0.000000,A=1.000000)" 9e+01)
  ;[1 1 1] reseau
  (Variables|Default|SetIsMyTurn? false)
  (bind _asbp_pmm_instance (Utilities|Casting|CastToBP_PMM_Instance (Game|GetGameInstance)))
  (CallFunction|SSpawnCharacterServer (Variables|/Game/CoreKlaft/BP_PMM_Instance.BP_PMM_Instance_C|GetCharacterSelection _asbp_pmm_instance) Controller))

(event Custom|S_SpawnCharacterServer
  (params (ClassCharacter :type BP%20Character%20Class%20Reference) (Target :type Controller%20Object%20Reference))
  ;[1 1 1] reseau
  (Development|PrintString "SpawnPlayerRunSercer" true true "(R=0.207907,G=1.000000,B=0.000000,A=1.000000)" 9e+01)
  (bind _outactors (Actor|GetAllActorsOfClass "/Script/Engine.PlayerStart"))
  (bind _array_element (Utilities|Array|ForEachLoopwithBreak _outactors :!label _label)
    (:LoopBody
      (if (Utilities|Name|NotEqual(Name) (Variables|/Script/Engine.PlayerStart|GetPlayerStartTag _array_element) "Found")
        (Variables|/Script/Engine.PlayerStart|SetPlayerStartTag _array_element "Found")
        (goto _label Break)))
    (:Completed
      (bind _returnvalue (Game|SpawnActorfromClass ClassCharacter (Math|Transform|MakeTransform (.location (Transformation|GetActorTransform _array_element)) (.rotation (Transformation|GetActorTransform _array_element)) "1,1,1") "AlwaysSpawn" 0 0 0))
      (Pawn|Possess self _returnvalue))))

(event EventTick
  (params (DeltaSeconds :type Float%20%28single-precision%29))
  (Development|PrintString (Utilities|String|ToString(Integer) (Variables|Default|GetIndexPlayer)) true true "(R=1.000000,G=0.908358,B=0.000000,A=1.000000)" 0.0))

(event EventBeginPlay
  (Input|SetInputModeGameOnly self)
  (EventDispatchers|BindEventtoOnActivePlayerSetIndex (.AsGMS%20Klaft (Utilities|Casting|CastToGMS_Klaft (Game|GetGameState))) (EventDispatchers|CreateEvent :!event PCKlaftGameAutoGenFunc)))

(event Input|MouseEvents|LeftMouseButton
  (params (Key :type Key%20Structure :default "None"))
  (:Pressed
    (if (Variables|Default|GetIsMyTurn?)
      (bind (_hitlocation _hittilecontenerref) (CallFunction|GetHitTilefromCursor))
      (if (Variables|/Game/Klaft/Blueprint/BP_TileContenerGrid.BP_TileContenerGrid_C|GetPOssibleToMove? _hittilecontenerref)
        (if (and (<= (Math|Vector|Distance(Vector) _hitlocation (Transformation|GetActorLocation (CallFunction|GetPlayerPawn))) 2e+02) (> (Math|Vector|Distance(Vector) _hitlocation (Transformation|GetActorLocation (CallFunction|GetPlayerPawn))) 75.0))
          (CallFunction|SLaunchAnimationTile _hittilecontenerref))))))

(event Custom|C_SetPlayerIndex
  (params (Index :type Integer))
  (Variables|Default|SetIndexPlayer Index)
  ;[0 0.976 1] Create widget Possible
  (bind _returnvalue (UserInterface|CreateWidget "/Game/CoreKlaft/WD_TestTourdejeu.WD_TestTourdejeu_C" 0 self (Variables|Default|GetIndexPlayer)))
  (UserInterface|Viewport|AddtoViewport _returnvalue 0))

(event Custom|S_FightSystemModule
  (params (RefEnemy :type BP%20Character%20Enemy%20Object%20Reference) (TileContenerRef :type BP%20Tile%20Contener%20Grid%20Object%20Reference))
  (bind _asbp_character (CallFunction|GetPlayerPawn))
  ;[1 1 1] MODULES
  ;;[1 1 1] Player Vs Mob
  (Utilities|IsValid RefEnemy
    (:Is%20Valid
      (Utilities|ModuleFight (Variables|/Game/CoreKlaft/BP_Character.BP_Character_C|GetRefInfoPlayer _asbp_character) (Variables|/Game/CoreKlaft/BP_CharacterEnemy.BP_CharacterEnemy_C|GetRefInfoEnemy RefEnemy)
        (:Win
          (Actor|DestroyActor RefEnemy)
          (CallFunction|SMovingPlayer (Transformation|GetActorLocation TileContenerRef)))
        (:Lose
          (Actor|DestroyActor _asbp_character))))))

(event Custom|S_LaunchAnimationTile
  (params (RefTileContener :type BP%20Tile%20Contener%20Grid%20Object%20Reference))
  (Default|SInitializeAnimTile RefTileContener self))

(event Custom|S_MovingPlayer
  (params (NewLocationPoint :type Vector))
  (Default|SMovingInializationAction (CallFunction|GetPlayerPawn) NewLocationPoint)
  (CallFunction|SPASystemModule))

(event Custom|S_ActionPlayer
  (params (Target :type BP%20Tile%20Contener%20Grid%20Object%20Reference))
  (bind _returnvalue (Transformation|GetActorLocation Target))
  (bind _asbp_character (CallFunction|GetPlayerPawn))
  (bind _returnvalue_2 (Transformation|GetActorLocation _asbp_character))
  (bind _returnvalue_3 (Math|Vector|Distance(Vector) _returnvalue _returnvalue_2))
  (if (Variables|/Game/Klaft/Blueprint/BP_TileContenerGrid.BP_TileContenerGrid_C|GetPOssibleToMove? Target)
    (if (and (<= _returnvalue_3 2e+02) (> _returnvalue_3 75.0))
      (CallFunction|SLaunchAnimationTile Target))))

(event Custom|S_EndPlayerTurn
  (Default|SEndPlayerTurn (.AsGMS%20Klaft (Utilities|Casting|CastToGMS_Klaft (Game|GetGameState)))))

(event Custom|Action
  (CallFunction|SPASystemModule))

(event Custom|S_PASystemModule
  (bind _asbp_character (CallFunction|GetPlayerPawn))
  ;[1 1 1] MODULES
  (if (== (.pa (Variables|/Game/CoreKlaft/BP_Character.BP_Character_C|GetPlayerInfoCurrentGame _asbp_character)) 0)
    (Variables|/Game/CoreKlaft/BP_Character.BP_Character_C|SetPlayerInfoCurrentGame _asbp_character (Utilities|Struct|MakeST_CaracPlayer2 (.posture (Variables|/Game/CoreKlaft/BP_Character.BP_Character_C|GetPlayerInfoCurrentGame _asbp_character)) (.attaque (Variables|/Game/CoreKlaft/BP_Character.BP_Character_C|GetPlayerInfoCurrentGame _asbp_character)) (.defense (Variables|/Game/CoreKlaft/BP_Character.BP_Character_C|GetPlayerInfoCurrentGame _asbp_character)) (.vitesse (Variables|/Game/CoreKlaft/BP_Character.BP_Character_C|GetPlayerInfoCurrentGame _asbp_character)) 0))
    (else
      (Variables|/Game/CoreKlaft/BP_Character.BP_Character_C|SetPlayerInfoCurrentGame _asbp_character (Utilities|Struct|MakeST_CaracPlayer2 (.posture (Variables|/Game/CoreKlaft/BP_Character.BP_Character_C|GetPlayerInfoCurrentGame _asbp_character)) (.attaque (Variables|/Game/CoreKlaft/BP_Character.BP_Character_C|GetPlayerInfoCurrentGame _asbp_character)) (.defense (Variables|/Game/CoreKlaft/BP_Character.BP_Character_C|GetPlayerInfoCurrentGame _asbp_character)) (.vitesse (Variables|/Game/CoreKlaft/BP_Character.BP_Character_C|GetPlayerInfoCurrentGame _asbp_character)) (- (.pa (Variables|/Game/CoreKlaft/BP_Character.BP_Character_C|GetPlayerInfoCurrentGame _asbp_character)) 1))))))

(fn ConstructionScript)

(fn PCKlaftGameAutoGenFunc
  (params (ActivePlayerIndex :type Integer))
  (if (== ActivePlayerIndex (Variables|Default|GetIndexPlayer))
    (Variables|Default|SetIsMyTurn? true)
    (else
      (Variables|Default|SetIsMyTurn? false))))

(fn GetHitTilefromCursor
  (bind _hitresult (Game|Player|GetHitResultUnderCursorbyChannel "TraceTypeQuery1" true))
  (bind (_bblockinghit _binitialoverlap _time _distance _location _impactpoint _normal _impactnormal _physmat _hitactor) (Collision|BreakHitResult _hitresult))
  (bind _asbp_tile_contener_grid (Utilities|Casting|CastToBP_TileContenerGrid (Actor|GetParentActor _hitactor))
    (:then
      (return _location _asbp_tile_contener_grid))
    (:CastFailed
      (return "0, 0, 0" 0))))

(fn GetPlayerPawn
  (bind _asbp_character (Utilities|Casting|CastToBP_Character (Pawn|GetControlledPawn)))
  (return _asbp_character))

(fn ResolutionBonusPosture
  (params (CaracPlayer :type ST%20Carac%20Player%202%20Structure) (CaracPlayer2 :type ST%20Carac%20Player%202%20Structure))
  (bind _valuebonusposture (Variables|Default|GetValueBonusPosture))
  (bind _valuebonusposture_2 (Variables|Default|GetValueBonusPosture))
  (Utilities|FlowControl|Sequence
    (:then_0
      ;[1 1 1] Player
      (bind _output_get (LocalVariables|SetL_CaracPlayer1 CaracPlayer))
      (LocalVariables|SetL_CaracPlayer1 (Utilities|Struct|MakeST_CaracPlayer2 (.posture (LocalVariables|GetL_CaracPlayer1)) (Utilities|Select :Index (.posture _output_get) :NewEnumerator0 (.attaque _output_get) :NewEnumerator1 (+ (.attaque _output_get) _valuebonusposture_2) :NewEnumerator2 (.attaque _output_get)) (Utilities|Select :Index (.posture _output_get) :NewEnumerator0 (+ (.defense _output_get) _valuebonusposture_2) :NewEnumerator1 (.defense _output_get) :NewEnumerator2 (.defense _output_get)) (Utilities|Select :Index (.posture _output_get) :NewEnumerator0 (.vitesse _output_get) :NewEnumerator1 (.vitesse _output_get) :NewEnumerator2 (+ (.vitesse _output_get) _valuebonusposture_2)) (.pa (LocalVariables|GetL_CaracPlayer1)))))
    (:then_1
      ;[1 1 1] Player2
      (bind _output_get_2 (LocalVariables|SetL_CaracPlayer2 CaracPlayer2))
      (LocalVariables|SetL_CaracPlayer2 (Utilities|Struct|MakeST_CaracPlayer2 (.posture (LocalVariables|GetL_CaracPlayer2)) (Utilities|Select :Index (.posture _output_get_2) :NewEnumerator0 (.attaque _output_get_2) :NewEnumerator1 (+ (.attaque _output_get_2) _valuebonusposture) :NewEnumerator2 (.attaque _output_get_2)) (Utilities|Select :Index (.posture _output_get_2) :NewEnumerator0 (+ (.defense _output_get_2) _valuebonusposture) :NewEnumerator1 (.defense _output_get_2) :NewEnumerator2 (.defense _output_get_2)) (Utilities|Select :Index (.posture _output_get_2) :NewEnumerator0 (.vitesse _output_get_2) :NewEnumerator1 (.vitesse _output_get_2) :NewEnumerator2 (+ (.vitesse _output_get_2) _valuebonusposture)) (.pa (LocalVariables|GetL_CaracPlayer2)))))
    (:then_2
      (return (LocalVariables|GetL_CaracPlayer1) (LocalVariables|GetL_CaracPlayer2)))))

(fn ResolutionCaracFight
  (params (CaracPlayer :type ST%20Carac%20Player%202%20Structure) (CaracPlayer2 :type ST%20Carac%20Player%202%20Structure))
  (LocalVariables|SetL_Player CaracPlayer)
  (LocalVariables|SetL_Player2 CaracPlayer2)
  (Utilities|FlowControl|Sequence
    (:then_0
      ;[1 1 1] Comment
      (LocalVariables|SetL_VitessePlayer (.Vitesse (Utilities|Struct|BreakST_CaracPlayer2 (LocalVariables|GetL_Player))))
      (LocalVariables|SetL_VitessePlayer2 (.Vitesse (Utilities|Struct|BreakST_CaracPlayer2 (LocalVariables|GetL_Player2)))))
    (:then_1
      ;[1 1 1] Comment
      (Math|Integer|CompareInt (.Vitesse (Utilities|Struct|BreakST_CaracPlayer2 (LocalVariables|GetL_Player))) (.Defense (Utilities|Struct|BreakST_CaracPlayer2 (LocalVariables|GetL_Player2)))
        (:>
          (LocalVariables|SetL_VitessePlayer (+ (LocalVariables|GetL_VitessePlayer) (.Vitesse (Utilities|Struct|BreakST_CaracPlayer2 (LocalVariables|GetL_Player))))))
        (:==)
        (:<
          (LocalVariables|SetL_VitessePlayer2 (+ (LocalVariables|GetL_VitessePlayer2) (.Defense (Utilities|Struct|BreakST_CaracPlayer2 (LocalVariables|GetL_Player2))))))))
    (:then_2
      ;[1 1 1] Comment
      (Math|Integer|CompareInt (.Defense (Utilities|Struct|BreakST_CaracPlayer2 (LocalVariables|GetL_Player))) (.Attaque (Utilities|Struct|BreakST_CaracPlayer2 (LocalVariables|GetL_Player2)))
        (:>
          (LocalVariables|SetL_VitessePlayer (+ (LocalVariables|GetL_VitessePlayer) (.Defense (Utilities|Struct|BreakST_CaracPlayer2 (LocalVariables|GetL_Player))))))
        (:==)
        (:<
          (LocalVariables|SetL_VitessePlayer2 (+ (LocalVariables|GetL_VitessePlayer2) (.Attaque (Utilities|Struct|BreakST_CaracPlayer2 (LocalVariables|GetL_Player2))))))))
    (:then_3
      (return (LocalVariables|GetL_VitessePlayer) (LocalVariables|GetL_VitessePlayer2)))))

(fn ResolutionBonusCard
  (params (CaracPlayer :type ST%20Carac%20Player%202%20Structure) (CaracPlayer2 :type ST%20Carac%20Player%202%20Structure) (BonusPlayer1 :type ST%20Carac%20Player%202%20Structure) (Bonus%20Player2 :type ST%20Carac%20Player%202%20Structure))
  (LocalVariables|SetL_CaractPlayer1 CaracPlayer)
  (LocalVariables|SetL_CaractPlayer2 CaracPlayer2)
  (LocalVariables|SetL_BonusPlayer1 BonusPlayer1)
  (LocalVariables|SetL_BonusPlayer2 Bonus%20Player2)
  (LocalVariables|SetL_CaractPlayer1 (Utilities|Struct|MakeST_CaracPlayer2 (.posture (LocalVariables|GetL_CaractPlayer1)) (+ (.attaque (LocalVariables|GetL_CaractPlayer1)) (.attaque (LocalVariables|GetL_BonusPlayer1))) (+ (.defense (LocalVariables|GetL_CaractPlayer1)) (.defense (LocalVariables|GetL_BonusPlayer1))) (+ (.vitesse (LocalVariables|GetL_CaractPlayer1)) (.vitesse (LocalVariables|GetL_BonusPlayer1))) (.pa (LocalVariables|GetL_CaractPlayer1))))
  (LocalVariables|SetL_CaractPlayer2 (Utilities|Struct|MakeST_CaracPlayer2 (.posture (LocalVariables|GetL_CaractPlayer2)) (+ (.attaque (LocalVariables|GetL_CaractPlayer2)) (.attaque (LocalVariables|GetL_BonusPlayer2))) (+ (.defense (LocalVariables|GetL_CaractPlayer2)) (.defense (LocalVariables|GetL_BonusPlayer2))) (+ (.vitesse (LocalVariables|GetL_CaractPlayer2)) (.vitesse (LocalVariables|GetL_BonusPlayer2))) (.pa (LocalVariables|GetL_CaractPlayer2))))
  (return (LocalVariables|GetL_CaractPlayer1) (LocalVariables|GetL_CaractPlayer2)))

(fn ResolutionBonusCoruption
  (params (CaracPlayer :type ST%20Carac%20Player%202%20Structure) (CaracPlayer2 :type ST%20Carac%20Player%202%20Structure))
  (return CaracPlayer CaracPlayer2))