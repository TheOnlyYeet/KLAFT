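; Enemy pawn Blueprint for the Klaft game that turns to face a target location, with server and multicast-style events relaying the rotation.
; A PawnMoving guard starts the move, then the AnimRotate timeline interpolates only yaw toward the target along the shortest path.
; Helpers for planar movement and timeline play rate exist but are not called here.
; The OnRep functions are empty, and turn-widget logic is disconnected.
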(event Custom|S_RotateEnemy
  (params (LocationTarget :type Vector))
  (CallFunction|MRotateEnemy LocationTarget))

(event Custom|M_RotateEnemy
  (params (LoctionTarget :type Vector))
  (if (not (Variables|Default|GetPawnMoving?))
    (Variables|Default|SetPawnMoving? true)
    (Variables|Default|SetLoctionPlayerTarget LoctionTarget)
    (Variables|Default|SetLocationPlayerStart (Transformation|GetActorLocation))
    (Variables|Default|SetRotationCameraStart (Transformation|GetActorRotation))
    ;[1 1 1] Step 1 : Rotation Pawn
    (bind _percentanim (Timeline|AnimRotate PlayFromStart)
      (:Update
        (CallFunction|SetrotationPawn _percentanim)))))

(fn ConstructionScript)

(fn SetLocationPawn
  (params (Alpha :type Float%20%28single-precision%29))
  (bind _loctionplayertarget (Variables|Default|GetLoctionPlayerTarget))
  (bind (_x _y) (Math|Vector|BreakVector _loctionplayertarget))
  (Transformation|SetActorLocation (Math|Vector|Lerp(Vector) (Variables|Default|GetLocationPlayerStart) (Math|Vector|MakeVector _x _y (.Z (Math|Vector|BreakVector (Variables|Default|GetLocationPlayerStart)))) Alpha) false false))

(fn SetrotationPawn
  (params (Alpha :type Float%20%28single-precision%29))
  (bind _rotationcamerastart (Variables|Default|GetRotationCameraStart))
  (Transformation|SetActorRotation (Math|Rotator|Lerp(Rotator) (Variables|Default|GetRotationCameraStart) (Math|Rotator|MakeRotator (.roll _rotationcamerastart) (.pitch _rotationcamerastart) (.yaw (Math|Rotator|FindLookatRotation (Variables|Default|GetLocationPlayerStart) (Variables|Default|GetLoctionPlayerTarget)))) Alpha true)))

(fn SetupTimeAnim
  (Components|Timeline|SetPlayRate (Variables|Default|GetAnimRotate) (/ 1.0 (Variables|Default|GetDurationAnimRotate))))

(fn OnRepInfoPlayer)

(fn OnRepPlayerInfoCurrentGame)

(fn OnRepIsMyTour?)

(fn OnRepNewVar0)