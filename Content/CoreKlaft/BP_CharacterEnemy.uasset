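; Enemy character in the Klaft game, using mage montages for combat, corruption, hit, death, victory and defeat reactions.
; S_ChangeAnimState picks a montage by state index, while S_RotateEnemy forwards a target to M_RotateEnemy.
; A timeline lerps yaw toward that target, switching StateAnim from Run to Idle; PawnMoving gates it but is never cleared here.
; Location-lerp and timeline-speed helpers are defined but uncalled here, and the OnRep handlers do nothing.
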(event Custom|S_ChangeAnimState
  (params (Index :type EListStateAnim%20Enum :default "NewEnumerator0"))
  (Animation|Montage|PlayMontage (Variables|Default|GetSkeletalMesh) (Utilities|Select :Index Index :NewEnumerator0 0 :NewEnumerator1 0 :NewEnumerator3 "/Game/LucasNayrac/Animation/Mage/Anim_Mage_EngagementCombat_Victoire_Montage.Anim_Mage_EngagementCombat_Victoire_Montage" :NewEnumerator2 "/Game/LucasNayrac/Animation/Mage/Anim_Mage_Mort_Montage.Anim_Mage_Mort_Montage" :NewEnumerator4 "/Game/LucasNayrac/Animation/Mage/Anim_Mage_PerdreCorruption_Montage.Anim_Mage_PerdreCorruption_Montage" :NewEnumerator5 "/Game/LucasNayrac/Animation/Mage/Anim_Mage_AspirerCorruption_Montage.Anim_Mage_AspirerCorruption_Montage" :NewEnumerator6 "/Game/LucasNayrac/Animation/Mage/Anim_Mage_Defaite_Montage.Anim_Mage_Defaite_Montage" :NewEnumerator7 "/Game/LucasNayrac/Animation/Mage/Anim_Mage_Victoire_Montage.Anim_Mage_Victoire_Montage" :NewEnumerator8 "/Game/LucasNayrac/Animation/Mage/Anim_Mage_Agonie_Montage.Anim_Mage_Agonie_Montage" :NewEnumerator9 "/Game/LucasNayrac/Animation/Mage/Anim_Mage_PrendreCoup_Montage.Anim_Mage_PrendreCoup_Montage" :NewEnumerator10 "/Game/LucasNayrac/Animation/Mage/Anim_Mage_DonnerCoup_Montage.Anim_Mage_DonnerCoup_Montage")))

(event Custom|S_RotateEnemy
  (params (LocationTarget :type Vector))
  (CallFunction|MRotateEnemy LocationTarget))

(event Custom|M_RotateEnemy
  (params (LoctionTarget :type Vector))
  (if (not (Variables|Default|GetPawnMoving?))
    (Variables|Default|SetPawnMoving? true)
    (Variables|Default|SetLoctionPlayerTarget LoctionTarget)
    (Variables|Default|SetLocationPlayerStart (Transformation|GetActorLocation))
    (Variables|Default|SetRotationCameraStart (Transformation|GetActorRotation))
    (Variables|Default|SetStateAnim "NewEnumerator1")
    ;[1 1 1] Step 1 : Rotation Pawn
    (bind _percentanim (Timeline|AnimRotate PlayFromStart)
      (:Update
        (CallFunction|SetrotationPawn _percentanim))
      (:Finished
        (Variables|Default|SetStateAnim "NewEnumerator0")))))

(fn ConstructionScript)

(fn SetLocationPawn
  (params (Alpha :type Float%20%28single-precision%29))
  (bind _loctionplayertarget (Variables|Default|GetLoctionPlayerTarget))
  (bind (_x _y) (Math|Vector|BreakVector _loctionplayertarget))
  (Transformation|SetActorLocation (Math|Vector|Lerp(Vector) (Variables|Default|GetLocationPlayerStart) (Math|Vector|MakeVector _x _y (.Z (Math|Vector|BreakVector (Variables|Default|GetLocationPlayerStart)))) Alpha) false false))

(fn SetrotationPawn
  (params (Alpha :type Float%20%28single-precision%29))
  (bind _rotationcamerastart (Variables|Default|GetRotationCameraStart))
  (Transformation|SetActorRotation (Math|Rotator|Lerp(Rotator) (Variables|Default|GetRotationCameraStart) (Math|Rotator|MakeRotator (.roll _rotationcamerastart) (.pitch _rotationcamerastart) (.yaw (Math|Rotator|FindLookatRotation (Variables|Default|GetLocationPlayerStart) (Variables|Default|GetLoctionPlayerTarget)))) Alpha true)))

(fn SetupTimeAnim
  (Components|Timeline|SetPlayRate (Variables|Default|GetAnimRotate) (/ 1.0 (Variables|Default|GetDurationAnimRotate))))

(fn OnRepInfoPlayer)

(fn OnRepPlayerInfoCurrentGame)

(fn OnRepIsMyTour?)

(fn OnRepNewVar0)

(fn OnRepStateAnim)