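; BP_GameInfo is a Blueprint that declares replicated match data: player controllers, found characters, player info and the index of the playing player.
; All OnRep handlers and the construction script are empty.
; Disconnected graph fragments would print BP_Character names, collect PC_KlaftGame controllers from the GameState PlayerArray, and roll a seeded random player index.
; None of that logic runs, so the asset currently has no active behavior of its own.
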(fn ConstructionScript)

(fn OnRepIndexPlayerPlay)

(fn OnRepRefPlayerController)

(fn OnRepRefPC)

(fn OnRepOutActors)

(fn OnRepInfoPlayer)