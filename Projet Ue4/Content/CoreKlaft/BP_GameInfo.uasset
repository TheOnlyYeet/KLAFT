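; BP_GameInfo is an unfinished game-info Blueprint for turn handling in the Klaft game.
; Live logic only prints its own name every Tick and provides S_PlayerController, which sets IsMyTour on the passed Target.
; Disconnected drafts gather characters and player controllers, give the second character the turn on authority, and roll a random player index.
; BeginPlay, M_PlayerController and all RepNotify handlers are empty.
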(event Custom|M_PlayerController)

(event Custom|S_PlayerController
  (params (Target :type BP%20Character%20Object%20Reference))
  (Variables|/Game/CoreKlaft/BP_Character.BP_Character_C|SetIsMyTour? Target true))

(event EventTick
  (params (DeltaSeconds :type Float%20%28single-precision%29))
  (Development|PrintString (Utilities|GetDisplayName self) true true "(R=0.000000,G=0.660000,B=1.000000,A=1.000000)" 0.0))

(event EventBeginPlay)

(fn ConstructionScript)

(fn OnRepIndexPlayerPlay)

(fn OnRepRefPlayerController)

(fn OnRepRefPC)

(fn OnRepOutActors)

(fn OnRepInfoPlayer)