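; Clickable map tile of a given type (forest, road, mountain, village, boss and others) on a grid.
; SetupTile sets the mesh from a data table row named after the type, then calls per-type defaults, which are an empty stub.
; Construction randomly rotates mountain meshes by 180 degrees.
; Clicking a tile within 200 units that the player is not on triggers RefGrid's animation if allowed; movement logic is unwired.
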(event MouseInput|EventActorOnClicked
  (params (ButtonPressed :type Key%20Structure :default "None"))
  (bind _refgrid (Variables|Default|GetrefGrid))
  (Development|PrintString "Hello" true true "(R=0.000000,G=1.000000,B=0.182792,A=1.000000)")
  (if (not (Math|Vector|Equal(Vector) (Transformation|GetActorLocation (Game|Player|GetPlayerPawn 0)) (Transformation|GetActorLocation) 5e+01))
    (if (<= (Math|Vector|Distance(Vector) (Transformation|GetActorLocation (Game|Player|GetPlayerPawn 0)) (Transformation|GetActorLocation)) 2e+02)
      (if (Variables|/Game/Klaft/Blueprint/BP_TileContenerGrid.BP_TileContenerGrid_C|GetAnimationPossible _refgrid)
        (Default|PlayAnimation _refgrid))
      (if (Variables|/Game/Klaft/Blueprint/BP_TileContenerGrid.BP_TileContenerGrid_C|GetPOssibleToMove? _refgrid)
        _))))

(fn ConstructionScript
  (if (Utilities|Enum|Equal(Enum) (Variables|Default|GetTypeTile) "NewEnumerator3")
    (Transformation|SetRelativeRotation (Variables|Default|GetStaticMesh) (select (Math|Random|RandomBool) "0,180.000000, 0" "0, 0, 0") false false)))

(fn GetDataTableInfoTile
  (bind _returnvalue (Utilities|GetDataTableRow (Variables|Default|GetDataInfo) (Utilities|String|StringToName (Utilities|String|EnumtoString (Variables|Default|GetTypeTile))))
    (:then
      _)
    (:RowNotFound
      _))
  (return _returnvalue))

(fn SettingsDefaultbyTypeTile
  (params (POssibleToMove? :type Boolean) (ClassMonter :type BP%20Character%20Class%20Reference) (PossibleMonster? :type Boolean))
  (Utilities|FlowControl|Sequence))

(fn SetupDefaultSettingsTille
  (switch Utilities|FlowControl|Switch|SwitchonEListTypeTile (Variables|Default|GetTypeTile)
    (:NewEnumerator0
      (CallFunction|SettingsDefaultbyTypeTile true 0 false))
    (:NewEnumerator1
      (CallFunction|SettingsDefaultbyTypeTile true 0 false))
    (:NewEnumerator2
      (CallFunction|SettingsDefaultbyTypeTile true 0 false))
    (:NewEnumerator3
      (CallFunction|SettingsDefaultbyTypeTile true 0 false))
    (:NewEnumerator4
      (CallFunction|SettingsDefaultbyTypeTile true 0 false))
    (:NewEnumerator5
      (CallFunction|SettingsDefaultbyTypeTile true 0 false))
    (:NewEnumerator6
      (CallFunction|SettingsDefaultbyTypeTile true 0 false))
    (:NewEnumerator7
      (CallFunction|SettingsDefaultbyTypeTile true 0 false))
    (:NewEnumerator8
      (CallFunction|SettingsDefaultbyTypeTile true 0 false))
    (:NewEnumerator9
      (CallFunction|SettingsDefaultbyTypeTile true 0 false))
    (:NewEnumerator10
      (CallFunction|SettingsDefaultbyTypeTile true 0 false))))

(fn SetupTile
  (params (TypeTile :type EListTypeTile%20Enum :default "NewEnumerator0"))
  (Variables|Default|SetTypeTile TypeTile)
  (Components|StaticMesh|SetStaticMesh (Variables|Default|GetStaticMesh) (Utilities|Array|Get(acopy) (.StaticMesh (Utilities|Struct|BreakST_TileInfo (CallFunction|GetDataTableInfoTile)))))
  (CallFunction|SetupDefaultSettingsTille))