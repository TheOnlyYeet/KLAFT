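; GM_Lobby is a lobby game mode that gathers players and sends the server to a random map once three have joined.
; On each PostLogin it adds the controller to ListPlayer and prints the player count.
; When the count equals three, it appends a random MapListForRandom entry to "ServerTravel" and runs the result as a console command.
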(event EventPostLogin
  (params (NewPlayer :type Player%20Controller%20Object%20Reference))
  (bind _listplayer (Variables|Default|GetListPlayer))
  (bind _returnvalue (Utilities|Array|Length _listplayer))
  (Utilities|Array|AddUnique _listplayer NewPlayer)
  (Development|PrintString (Utilities|String|ToString(Integer) _returnvalue))
  (if (== _returnvalue 3)
    (Development|ExecuteConsoleCommand (Utilities|String|Append "ServerTravel " (.OutItem (Utilities|Array|Random (Variables|Default|GetMapListForRandom)))) 0)))

(fn ConstructionScript)