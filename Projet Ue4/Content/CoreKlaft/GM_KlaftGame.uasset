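; Game mode for KlaftGame, a turn-based tile game that registers joining players and spawns their pawns at unclaimed PlayerStarts.
; Rounds ("Manch") rotate through three controllers in order, loading the active character's stats.
; Each action spends an action point to move toward a nearby tile under the cursor, and exhausted points end the turn.
; An unwired fight module resolves posture bonuses, pass-through card bonuses and stat comparisons, only printing the outcome.
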(event Custom|SpawnCharacter
  (params (Target :type Controller%20Object%20Reference) (NewParam :type BP%20Character%20Class%20Reference))
  (bind _returnvalue (Pawn|GetControlledPawn Target))
  (bind _outactors (Actor|GetAllActorsOfClass "/Script/Engine.PlayerStart"))
  (bind _array_element (Utilities|Array|ForEachLoopwithBreak _outactors :!label _label)
    (:LoopBody
      (if (Utilities|Name|NotEqual(Name) (Variables|/Script/Engine.PlayerStart|GetPlayerStartTag _array_element) "Found")
        (Variables|/Script/Engine.PlayerStart|SetPlayerStartTag _array_element "Found")
        (goto _label Break)))
    (:Completed
      (Utilities|IsValid _returnvalue
        (:Is%20Valid
          (Actor|DestroyActor _returnvalue))
        (:Is%20Not%20Valid
          _))
      (bind _returnvalue_2 (Game|SpawnActorfromClass NewParam (Math|Transform|MakeTransform (.location (Transformation|GetActorTransform _array_element)) (.rotation (Transformation|GetActorTransform _array_element)) "1,1,1") "Undefined" 0 0 0))
      (Pawn|Possess Target _returnvalue_2))))

(event EventPostLogin
  (params (NewPlayer :type Player%20Controller%20Object%20Reference))
  (bind _returnvalue (Utilities|Array|AddUnique (Variables|Default|GetNew%20Player) NewPlayer))
  (Variables|/Game/CoreKlaft/BP_PMM_Instance.BP_PMM_Instance_C|SetIndexPlayer (.AsBP%20PMM%20Instance (Utilities|Casting|CastToBP_PMM_Instance (Game|GetGameInstance))) _returnvalue)
  (bind _aspc_klaft_game (Utilities|Casting|CastToPC_KlaftGame NewPlayer))
  (Default|CSpawnCharacter _aspc_klaft_game 0 NewPlayer))

(event Custom|LaunchParty
  ;[0.3886 1 0.009875] PHASE : NewPartyLaunch
  (CallFunction|OrderOfPlay)
  (CallFunction|StartManchEvent))

(event Custom|StartManchEvent
  ;[0.3802 0.7216 1] PHASE : Start Manch
  (CallFunction|InitialisationStartManchPlayer))

(event Custom|EndManchEvent
  ;[0 0.05833 0.1059] PHASE : End Manch
  (CallFunction|InitializationNewIndexPlayer)
  (CallFunction|StartManchEvent))

(event Custom|ActionControllerPlayer
  (Development|PrintString "Hello")
  (CallFunction|MovingPhase))

(event Custom|MovingPhase
  ;[0 0.5508 1] PHASE : Moving
  (bind _dispopa_ (CallFunction|PAModule))
  (if _dispopa_
    (CallFunction|MoveAction)
    (else
      (CallFunction|EndManchEvent))))

(event EventBeginPlay
  (CallFunction|StartManchEvent))

(fn ConstructionScript)

(fn PAModule
  (if (== (.pa (Variables|Default|GetCaracPlayer)) 0)
    (return false)
    (else
      (Variables|Default|SetCaracPlayer (Utilities|Struct|MakeST_CaracPlayer2 (.posture (Variables|Default|GetCaracPlayer)) (.attaque (Variables|Default|GetCaracPlayer)) (.defense (Variables|Default|GetCaracPlayer)) (.vitesse (Variables|Default|GetCaracPlayer)) (- (.pa (Variables|Default|GetCaracPlayer)) 1)))
      (return true))))

(fn FightModule
  (bind (_newcaracplayer _newcaracplayer2) (CallFunction|ResolutionBonusPosture (Variables|Default|GetCaracPlayer) (Variables|Default|GetCaracPlayer2)))
  (bind (_newcaracplayer_2 _newcaracplayer2_2) (CallFunction|ResolutionBonusCard _newcaracplayer _newcaracplayer2))
  (bind (_l_vitesseplayer1 _l_vitesseplayer21) (CallFunction|ResolutionCaracFight _newcaracplayer_2 _newcaracplayer2_2))
  (Math|Integer|CompareInt _l_vitesseplayer1 _l_vitesseplayer21
    (:>
      (Development|PrintString "WIn !" true true "(R=0.193532,G=1.000000,B=0.000000,A=1.000000)"))
    (:==
      (Development|PrintString "Equal" true true "(R=0.968520,G=1.000000,B=0.000000,A=1.000000)"))
    (:<
      (Development|PrintString "Lose" true true "(R=1.000000,G=0.000000,B=0.064907,A=1.000000)"))))

(fn ResolutionBonusPosture
  (params (CaracPlayer :type ST%20Carac%20Player%202%20Structure) (CaracPlayer2 :type ST%20Carac%20Player%202%20Structure))
  (bind _valuebonusposture (Variables|Default|GetValueBonusPosture))
  (bind _valuebonusposture_2 (Variables|Default|GetValueBonusPosture))
  (Utilities|FlowControl|Sequence
    (:then_0
      ;[1 1 1] Player
      (bind _output_get (LocalVariables|SetL_CaracPlayer1 CaracPlayer))
      (LocalVariables|SetL_CaracPlayer1 (Utilities|Struct|MakeST_CaracPlayer2 (.posture (LocalVariables|GetL_CaracPlayer1)) (Utilities|Select :Index (.posture _output_get) :NewEnumerator0 (.attaque _output_get) :NewEnumerator1 (+ (.attaque _output_get) _valuebonusposture_2) :NewEnumerator2 (.attaque _output_get)) (Utilities|Select :Index (.posture _output_get) :NewEnumerator0 (+ (.defense _output_get) _valuebonusposture_2) :NewEnumerator1 (.defense _output_get) :NewEnumerator2 (.defense _output_get)) (Utilities|Select :Index (.posture _output_get) :NewEnumerator0 (.vitesse _output_get) :NewEnumerator1 (.vitesse _output_get) :NewEnumerator2 (+ (.vitesse _output_get) _valuebonusposture_2)) (.pa (LocalVariables|GetL_CaracPlayer1)))))
    (:then_1
      ;[1 1 1] Player2
      (bind _output_get_2 (LocalVariables|SetL_CaracPlayer2 CaracPlayer2))
      (LocalVariables|SetL_CaracPlayer2 (Utilities|Struct|MakeST_CaracPlayer2 (.posture (LocalVariables|GetL_CaracPlayer2)) (Utilities|Select :Index (.posture _output_get_2) :NewEnumerator0 (.attaque _output_get_2) :NewEnumerator1 (+ (.attaque _output_get_2) _valuebonusposture) :NewEnumerator2 (.attaque _output_get_2)) (Utilities|Select :Index (.posture _output_get_2) :NewEnumerator0 (+ (.defense _output_get_2) _valuebonusposture) :NewEnumerator1 (.defense _output_get_2) :NewEnumerator2 (.defense _output_get_2)) (Utilities|Select :Index (.posture _output_get_2) :NewEnumerator0 (.vitesse _output_get_2) :NewEnumerator1 (.vitesse _output_get_2) :NewEnumerator2 (+ (.vitesse _output_get_2) _valuebonusposture)) (.pa (LocalVariables|GetL_CaracPlayer2)))))
    (:then_2
      (return (LocalVariables|GetL_CaracPlayer1) (LocalVariables|GetL_CaracPlayer2)))))

(fn ResolutionCaracFight
  (params (CaracPlayer :type ST%20Carac%20Player%202%20Structure) (CaracPlayer2 :type ST%20Carac%20Player%202%20Structure))
  (LocalVariables|SetL_Player CaracPlayer)
  (LocalVariables|SetL_Player2 CaracPlayer2)
  (Utilities|FlowControl|Sequence
    (:then_0
      ;[1 1 1] Comment
      (LocalVariables|SetL_VitessePlayer (.Vitesse (Utilities|Struct|BreakST_CaracPlayer2 (LocalVariables|GetL_Player))))
      (LocalVariables|SetL_VitessePlayer2 (.Vitesse (Utilities|Struct|BreakST_CaracPlayer2 (LocalVariables|GetL_Player2)))))
    (:then_1
      ;[1 1 1] Comment
      (Math|Integer|CompareInt (.Vitesse (Utilities|Struct|BreakST_CaracPlayer2 (LocalVariables|GetL_Player))) (.Defense (Utilities|Struct|BreakST_CaracPlayer2 (LocalVariables|GetL_Player2)))
        (:>
          (LocalVariables|SetL_VitessePlayer (+ (LocalVariables|GetL_VitessePlayer) (.Vitesse (Utilities|Struct|BreakST_CaracPlayer2 (LocalVariables|GetL_Player))))))
        (:==)
        (:<
          (LocalVariables|SetL_VitessePlayer2 (+ (LocalVariables|GetL_VitessePlayer2) (.Defense (Utilities|Struct|BreakST_CaracPlayer2 (LocalVariables|GetL_Player2))))))))
    (:then_2
      ;[1 1 1] Comment
      (Math|Integer|CompareInt (.Defense (Utilities|Struct|BreakST_CaracPlayer2 (LocalVariables|GetL_Player))) (.Attaque (Utilities|Struct|BreakST_CaracPlayer2 (LocalVariables|GetL_Player2)))
        (:>
          (LocalVariables|SetL_VitessePlayer (+ (LocalVariables|GetL_VitessePlayer) (.Defense (Utilities|Struct|BreakST_CaracPlayer2 (LocalVariables|GetL_Player))))))
        (:==)
        (:<
          (LocalVariables|SetL_VitessePlayer2 (+ (LocalVariables|GetL_VitessePlayer2) (.Attaque (Utilities|Struct|BreakST_CaracPlayer2 (LocalVariables|GetL_Player2))))))))
    (:then_3
      (return (LocalVariables|GetL_VitessePlayer) (LocalVariables|GetL_VitessePlayer2)))))

(fn ResolutionBonusCard
  (params (CaracPlayer :type ST%20Carac%20Player%202%20Structure) (CaracPlayer2 :type ST%20Carac%20Player%202%20Structure))
  (return CaracPlayer CaracPlayer2))

(fn InitialisationStartManchPlayer
  (bind _indexcontrollerisplay (Variables|Default|GetIndexControllerIsPlay))
  (bind _order (Variables|Default|GetOrder))
  (bind _output (Utilities|Array|Get(acopy) _order _indexcontrollerisplay))
  (Variables|Default|SetRefControllerIsPlayed _output)
  (Variables|Default|SetCaracPlayer (Variables|/Game/CoreKlaft/BP_Character.BP_Character_C|GetInfoPlayer (.AsBP%20Character (Utilities|Casting|CastToBP_Character (Pawn|GetControlledPawn (Variables|Default|GetRefControllerIsPlayed))))))
  (Development|PrintString (Utilities|GetDisplayName _output)))

(fn OrderOfPlay
  (bind _output_get (LocalVariables|SetNewLocalVar_1 (Variables|Default|GetNew%20Player)))
  ;[1 1 1] Comment
  (Variables|Default|SetIndexControllerIsPlay 0)
  (Variables|Default|SetOrder _output_get))

(fn InitializationNewIndexPlayer
  (Variables|/Game/CoreKlaft/PC_KlaftGame.PC_KlaftGame_C|SetMyManch? (.AsPC%20Klaft%20Game (Utilities|Casting|CastToPC_KlaftGame (Utilities|Array|Get(acopy) (Variables|Default|GetOrder) (Variables|Default|GetIndexControllerIsPlay)))) false)
  ;[1 1 1] NextIndexPlayer
  (if (== (Variables|Default|GetIndexControllerIsPlay) 2)
    (Variables|Default|SetIndexControllerIsPlay 0)
    (else
      (Variables|Default|SetIndexControllerIsPlay (+ (Variables|Default|GetIndexControllerIsPlay) 1))))
  (Variables|/Game/CoreKlaft/PC_KlaftGame.PC_KlaftGame_C|SetMyManch? (.AsPC%20Klaft%20Game (Utilities|Casting|CastToPC_KlaftGame (Utilities|Array|Get(acopy) (Variables|Default|GetOrder) (Variables|Default|GetIndexControllerIsPlay)))) true))

(fn MoveAction
  (bind _refcontrollerisplayed (Variables|Default|GetRefControllerIsPlayed))
  (bind _hitresult (Game|Player|GetHitResultUnderCursorbyChannel _refcontrollerisplayed "TraceTypeQuery1" true))
  (bind _asbp_character (Utilities|Casting|CastToBP_Character (Pawn|GetControlledPawn (Variables|Default|GetRefControllerIsPlayed))))
  (if (not (Variables|/Game/CoreKlaft/BP_Character.BP_Character_C|GetPawnMoving? _asbp_character))
    (bind _asbp_tileversoin_2 (Utilities|Casting|CastToBP_Tileversoin2 (.hitactor _hitresult)))
    (if (<= (Math|Vector|Distance(Vector) (.location _hitresult) (Transformation|GetActorLocation _asbp_character)) 2e+02)
      (Default|SMovingInializationAction _asbp_character (Transformation|GetActorLocation _asbp_tileversoin_2)))))