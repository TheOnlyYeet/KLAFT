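; BP_LimitMap is an actor that, judging by its name, marks the limits of the playable map.
; On BeginPlay it reads its own actor bounds, including non-colliding components, and adds or subtracts the box extent from the origin on each axis.
; The results are stored as min and max variables for X, Y and Z, with no clamping or enforcement in this Blueprint.
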(event EventBeginPlay
  (bind (_origin _boxextent) (Collision|GetActorBounds false false))
  (bind (_x _y _z) (Math|Vector|BreakVector _origin))
  (bind (_x_2 _y_2 _z_2) (Math|Vector|BreakVector _boxextent))
  (Utilities|FlowControl|Sequence
    (:then_0
      (Variables|Default|SetXmax (+ _x _x_2)))
    (:then_1
      (Variables|Default|SetXmin (- _x _x_2)))
    (:then_2
      (Variables|Default|SetYmax (+ _y _y_2)))
    (:then_3
      (Variables|Default|SetYmin (- _y _y_2)))
    (:then_4
      (Variables|Default|SetZmax (+ _z _z_2)))
    (:then_5
      (Variables|Default|SetZmin (- _z _z_2)))))

(fn ConstructionScript)